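; Destructible abbey window Blueprint that shatters when damaged by a bomb.
; Damage from a BombBP applies radius damage to the destructible mesh using the bomb's impulse range, unless it has already fractured.
; The same hit is forwarded to the closest Window_01_Glass_DM_BP within a small radius, so nearby glass breaks with it.
; On fracture, it destroys itself after the GameInstance's chunk lifetime, if positive.
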(event Custom|OnActorFracture_Event_0
  (params (HitPoint :type Vector%20%28by%20ref%29) (HitDirection :type Vector%20%28by%20ref%29))
  (Variables|Default|SetHasFractured true)
  (bind _asskele_game_instance (Utilities|Casting|CastToSkele_GameInstance (Game|GetGameInstance)))
  (if (> (Variables|/Game/SkeletonWar/Blueprints/Skele_GameInstance.Skele_GameInstance_C|GetChunkLifetime _asskele_game_instance) 0.0)
    (Utilities|FlowControl|Delay (Variables|/Game/SkeletonWar/Blueprints/Skele_GameInstance.Skele_GameInstance_C|GetChunkLifetime _asskele_game_instance))
    (Actor|DestroyActor)))

(event Custom|DamageObject
  (params (Damage :type Float%20%28single-precision%29) (Origin :type Vector) (DamageRadius :type Float%20%28single-precision%29))
  (if (not (Variables|Default|GetHasFractured))
    (Class|DestructibleComponent|ApplyRadiusDamage (Variables|Default|GetDestructibleComponent) Damage Origin DamageRadius 2e+02 true)))

(event Collision|EventActorBeginOverlap
  (params (OtherActor :type Actor%20Object%20Reference)))

(event EventTick
  (params (DeltaSeconds :type Float%20%28single-precision%29)))

(event Game|Damage|EventAnyDamage
  (params (Damage :type Float%20%28single-precision%29) (DamageType :type Damage%20Type%20Object%20Reference) (InstigatedBy :type Controller%20Object%20Reference) (DamageCauser :type Actor%20Object%20Reference))
  (bind _returnvalue (Transformation|GetActorLocation DamageCauser))
  (bind _self self)
  (bind (_isvalid _returnvalue_2) (Class|VictoryBPFunctionLibrary|GetClosestActorOfClassinRadiusOfActor "/Game/SkeletonWar/StaticMeshes/Abbey/Window_01_Glass_DM_BP.Window_01_Glass_DM_BP_C" _self 1e+02))
  (bind _asbomb_bp (Utilities|Casting|CastToBombBP DamageCauser))
  (CallFunction|DamageObject Damage _returnvalue (Variables|/Game/SkeletonWar/Blueprints/Weapons/BombBP.BombBP_C|GetBombImpulseRange _asbomb_bp))
  (if _isvalid
    (bind _aswindow_01_glass_dm_bp (Utilities|Casting|CastToWindow_01_Glass_DM_BP _returnvalue_2))
    (Default|DamageObject _aswindow_01_glass_dm_bp Damage _returnvalue (Variables|/Game/SkeletonWar/Blueprints/Weapons/BombBP.BombBP_C|GetBombImpulseRange _asbomb_bp))))

(event EventBeginPlay
  (Variables|Default|SetHasFractured false)
  (EventDispatchers|AssignOnActorFracture (delegate Custom|OnActorFracture_Event_0)))

(fn ConstructionScript)