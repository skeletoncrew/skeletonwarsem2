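; Destructible abbey window glass Blueprint for Skeleton War that shatters when hit by bomb damage.
; Damage from a BombBP applies radius damage to the destructible component using the bomb's impulse range and plays a glass smash sound, but only until it fractures.
; On fracture it sets a flag and, if the game instance's ChunkLifetime is positive, destroys itself after that delay.
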(event Custom|OnActorFracture_Event_0
  (params (HitPoint :type Vector%20%28by%20ref%29) (HitDirection :type Vector%20%28by%20ref%29))
  (Variables|Default|SetHasFractured true)
  (bind _asskele_game_instance (Utilities|Casting|CastToSkele_GameInstance (Game|GetGameInstance)))
  (if (> (Variables|/Game/SkeletonWar/Blueprints/Skele_GameInstance.Skele_GameInstance_C|GetChunkLifetime _asskele_game_instance) 0.0)
    (Utilities|FlowControl|Delay (Variables|/Game/SkeletonWar/Blueprints/Skele_GameInstance.Skele_GameInstance_C|GetChunkLifetime _asskele_game_instance))
    (Actor|DestroyActor)))

(event Custom|DamageObject
  (params (Damage :type Float%20%28single-precision%29) (Origin :type Vector) (DamageRadius :type Float%20%28single-precision%29))
  (if (not (Variables|Default|GetHasFractured))
    (Class|DestructibleComponent|ApplyRadiusDamage (Variables|Default|GetDestructibleComponent) Damage Origin DamageRadius 2e+02 true)
    (Audio|PlaySoundatLocation "/Game/SkeletonWar/Sounds/BombCollision/GlassSmashCue.GlassSmashCue" (Transformation|GetActorLocation))))

(event Game|Damage|EventAnyDamage
  (params (Damage :type Float%20%28single-precision%29) (DamageType :type Damage%20Type%20Object%20Reference) (InstigatedBy :type Controller%20Object%20Reference) (DamageCauser :type Actor%20Object%20Reference))
  (bind _asbomb_bp (Utilities|Casting|CastToBombBP DamageCauser))
  (CallFunction|DamageObject Damage (Transformation|GetActorLocation DamageCauser) (Variables|/Game/SkeletonWar/Blueprints/Weapons/BombBP.BombBP_C|GetBombImpulseRange _asbomb_bp)))

(event Collision|EventActorBeginOverlap
  (params (OtherActor :type Actor%20Object%20Reference)))

(event EventTick
  (params (DeltaSeconds :type Float%20%28single-precision%29)))

(event EventBeginPlay
  (Variables|Default|SetHasFractured false)
  (EventDispatchers|AssignOnActorFracture (delegate Custom|OnActorFracture_Event_0)))

(fn ConstructionScript)