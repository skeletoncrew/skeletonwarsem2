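; Skeleton War game mode that handles player login, respawning and Rubix-mode colour assignment.
; On login it numbers and names players and copies server settings from the game instance to the game state.
; Respawns spawn and possess a Skele_BP at the PlayerStart farthest from its nearest skeleton, or randomly when alone.
; Rubix mode colours skeletons by player and scrambles limb colours, using per-type non-matching limb arrays to swap colours.
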(event Custom|Respawn
  (params (Controller :type Player%20Controller%20Object%20Reference))
  ;[1 1 1] Pick a respawn point and possess a new pawn
  (Utilities|IsValid Controller
    (:Is%20Valid
      (Networking|SwitchHasAuthority
        (:Authority
          (bind _transform (CallFunction|GetSafestRespawnPoint))
          (bind _returnvalue (Game|SpawnActorfromClass "/Game/SkeletonWar/Blueprints/PlayerCharacters/Skele_BP.Skele_BP_C" _transform true Controller 0))
          (Utilities|IsValid _returnvalue
            (:Is%20Valid
              (Pawn|Possess Controller _returnvalue))))))))

(event EventPostLogin
  (params (NewPlayer :type Player%20Controller%20Object%20Reference))
  ;[1 1 1] Set the player's name and call the PostLogin event
  (bind _asskele_player_controller (Utilities|Casting|CastToSkele_PlayerController NewPlayer))
  (Variables|/Game/SkeletonWar/Blueprints/Skele_PlayerController.Skele_PlayerController_C|SetPlayerNumber _asskele_player_controller (Variables|Default|GetNumPlayers))
  (Networking|SwitchHasAuthority
    (:Authority
      (bind _asskele_player_state (Utilities|Casting|CastToSkele_PlayerState (Variables|/Script/Engine.Controller|GetPlayerState NewPlayer)))
      (bind _asskele_game_instance (Utilities|Casting|CastToSkele_GameInstance (Game|GetGameInstance)))
      (bind _asskele_game_state (Utilities|Casting|CastToSkele_GameState (Game|GetGameState))
        (:then
          (Variables|/Game/SkeletonWar/Blueprints/Skele_GameState.Skele_GameState_C|SetGameEndTime _asskele_game_state (* (.GameTime (Utilities|Struct|BreakServerSettings_Struct (Variables|/Game/SkeletonWar/Blueprints/Skele_GameInstance.Skele_GameInstance_C|GetServerSettings _asskele_game_instance))) 6e+01))
          (Variables|/Game/SkeletonWar/Blueprints/Skele_GameState.Skele_GameState_C|SetServerName _asskele_game_state (.ServerName (Utilities|Struct|BreakServerSettings_Struct (Variables|/Game/SkeletonWar/Blueprints/Skele_GameInstance.Skele_GameInstance_C|GetServerSettings _asskele_game_instance))))
          (Utilities|Array|Clear (Variables|Default|GetPlayerNamesTemp))
          (for _array_element (Variables|/Game/SkeletonWar/Blueprints/Skele_GameState.Skele_GameState_C|GetSkelePlayerStates _asskele_game_state)
            (Utilities|Array|Add (Variables|Default|GetPlayerNamesTemp) (Variables|/Game/SkeletonWar/Blueprints/Skele_PlayerState.Skele_PlayerState_C|GetCurrentPlayerName _array_element)))
          (Variables|/Game/SkeletonWar/Blueprints/Skele_PlayerState.Skele_PlayerState_C|SetCurrentPlayerName _asskele_player_state (Class|SkeleUtilityFunctionLibrary|GetPlayerNamewithSuffix 0 (Variables|/Game/SkeletonWar/Blueprints/Skele_GameInstance.Skele_GameInstance_C|GetPlayerName _asskele_game_instance))))
        (:CastFailed
          (Variables|/Game/SkeletonWar/Blueprints/Skele_PlayerState.Skele_PlayerState_C|SetCurrentPlayerName _asskele_player_state (Variables|/Game/SkeletonWar/Blueprints/Skele_GameInstance.Skele_GameInstance_C|GetPlayerName _asskele_game_instance))))
      (bind _asskele_player_controller_2 (Utilities|Casting|CastToSkele_PlayerController NewPlayer))
      (Default|ClientPostLogin _asskele_player_controller_2))))

(event Custom|AssignColour
  (params (Bone :type Actor%20Object%20Reference))
  ;[1 1 1] If it's rubix mode set colour
  (Networking|SwitchHasAuthority
    (:Authority
      (if (Utilities|Enum|Equal(Enum) (Variables|Default|GetGameMode) "NewEnumerator1")
        (CallFunction|SetColour Bone)))))

(fn ConstructionScript
  ;[1 1 1] Set the game mode
  (bind _asskele_game_instance (Utilities|Casting|CastToSkele_GameInstance (Game|GetGameInstance)))
  (Variables|Default|SetGameMode (.GameMode (Utilities|Struct|BreakServerSettings_Struct (Variables|/Game/SkeletonWar/Blueprints/Skele_GameInstance.Skele_GameInstance_C|GetServerSettings _asskele_game_instance)))))

(fn SetColour
  (params (Actor :type Actor%20Object%20Reference))
  (bind _numplayers (Variables|Default|GetNumPlayers))
  (bind _arrayofints (Variables|Default|GetArrayofInts))
  (bind _numplayers_2 (Variables|Default|GetNumPlayers))
  (bind _returnvalue (- _numplayers_2 1))
  (bind _asskele_bp (Utilities|Casting|CastToSkele_BP Actor)
    (:then
      (bind _asskele_player_controller (Utilities|Casting|CastToSkele_PlayerController (Components|GetOwner _asskele_bp))
        (:then
          (Variables|/Game/SkeletonWar/Blueprints/PlayerCharacters/Skele_BP.Skele_BP_C|SetColourIndex _asskele_bp (- (Variables|/Game/SkeletonWar/Blueprints/Skele_PlayerController.Skele_PlayerController_C|GetPlayerNumber _asskele_player_controller) 1))
          (Variables|Rubix|SetTempPlayerColourIndex (- (Variables|/Game/SkeletonWar/Blueprints/Skele_PlayerController.Skele_PlayerController_C|GetPlayerNumber _asskele_player_controller) 1))
          (if (Variables|Default|GetPlayer1Setup)
            (Variables|Default|SetFirstSetUp true)))
        (:CastFailed
          (Variables|/Game/SkeletonWar/Blueprints/PlayerCharacters/Skele_BP.Skele_BP_C|SetColourIndex _asskele_bp _returnvalue)
          (Variables|Rubix|SetTempPlayerColourIndex _returnvalue))))
    (:CastFailed
      (bind _aslimb_2 (Utilities|Casting|CastToLimb2 Actor))
      (if (Variables|Default|GetFirstSetUp)
        (Utilities|Array|RemoveItem _arrayofints (Variables|Rubix|GetTempPlayerColourIndex))
        (Variables|/Game/SkeletonWar/Blueprints/Limbs/Limb2.Limb2_C|SetColourIndex _aslimb_2 (Utilities|Array|Get(acopy) _arrayofints (Math|Random|RandomIntegerinRange 0 (- (Variables|Default|GetNumPlayers) 2))))
        (Utilities|Array|Insert _arrayofints (Variables|Rubix|GetTempPlayerColourIndex) (Variables|Rubix|GetTempPlayerColourIndex))
        (elif (== _numplayers 1)
          (Variables|/Game/SkeletonWar/Blueprints/Limbs/Limb2.Limb2_C|SetColourIndex _aslimb_2 1)
          (Variables|Default|SetPlayer1Setup true)
          (elif (== _numplayers 2)
            (Variables|/Game/SkeletonWar/Blueprints/Limbs/Limb2.Limb2_C|SetColourIndex _aslimb_2 0)
            (elif (>= _numplayers 3)
              (if (< (Utilities|Array|Length (Variables|Rubix|GetNonMatchingLimbs)) 1)
                (Variables|/Game/SkeletonWar/Blueprints/Limbs/Limb2.Limb2_C|SetColourIndex _aslimb_2 (Variables|Rubix|GetTempPlayerColourIndex))
                (else
                  (bind _ashead_bp (Utilities|Casting|CastToHead_BP _aslimb_2)
                    (:then
                      (CallFunction|SetIndexfromNonMatchingLimbArray _ashead_bp (Variables|Rubix|GetHead)))
                    (:CastFailed
                      (bind _asleft_arm_bp (Utilities|Casting|CastToLeftArm_BP _aslimb_2)
                        (:then
                          (CallFunction|SetIndexfromNonMatchingLimbArray _asleft_arm_bp (Variables|Rubix|GetLeftArm)))
                        (:CastFailed
                          (bind _asright_arm_bp (Utilities|Casting|CastToRightArm_BP _aslimb_2)
                            (:then
                              (CallFunction|SetIndexfromNonMatchingLimbArray _asright_arm_bp (Variables|Rubix|GetRightArm)))
                            (:CastFailed
                              (bind _asleft_leg_bp (Utilities|Casting|CastToLeftLeg_BP _aslimb_2)
                                (:then
                                  (CallFunction|SetIndexfromNonMatchingLimbArray _asleft_leg_bp (Variables|Rubix|GetLeftLeg)))
                                (:CastFailed
                                  (bind _asright_leg_bp (Utilities|Casting|CastToRightLeg_BP _aslimb_2))
                                  (CallFunction|SetIndexfromNonMatchingLimbArray _asright_leg_bp (Variables|Rubix|GetRightLeg)))))))))))))))))))

(fn SetIndexfromNonMatchingLimbArray
  (params (Limb :type Limb%202%20Object%20Reference) (NonMatchingLimbArray :type Array%20of%20Limb%202%20Object%20References))
  (if (Utilities|ArrayNotEmpty NonMatchingLimbArray)
    (bind _output_get (Variables|Rubix|SetTempArrayIndex (Math|Random|RandomInteger (Utilities|Array|Length NonMatchingLimbArray))))
    (bind _output_get_2 (Variables|Rubix|SetTempColourIndex (Variables|/Game/SkeletonWar/Blueprints/Limbs/Limb2.Limb2_C|GetColourIndex (Utilities|Array|Get(acopy) NonMatchingLimbArray _output_get))))
    (Variables|/Game/SkeletonWar/Blueprints/Limbs/Limb2.Limb2_C|SetColourIndex (Utilities|Array|Get(acopy) NonMatchingLimbArray _output_get) (Variables|Rubix|GetTempPlayerColourIndex))
    (Variables|/Game/SkeletonWar/Blueprints/Limbs/Limb2.Limb2_C|SetColourIndex Limb _output_get_2)
    (else
      (Variables|/Game/SkeletonWar/Blueprints/Limbs/Limb2.Limb2_C|SetColourIndex Limb (Variables|Rubix|GetTempPlayerColourIndex)))))

(fn AddtoNonMatchingLimbArrays
  (params (Limb :type Limb%202%20Object%20Reference))
  (bind _nonmatchinglimbs (Variables|Rubix|GetNonMatchingLimbs))
  (if (not (Utilities|Array|ContainsItem _nonmatchinglimbs Limb))
    (Utilities|Array|Add _nonmatchinglimbs Limb)
    (bind _ashead_bp (Utilities|Casting|CastToHead_BP Limb)
      (:then
        (Utilities|Array|Add (Variables|Rubix|GetHead) _ashead_bp))
      (:CastFailed
        (bind _asleft_arm_bp (Utilities|Casting|CastToLeftArm_BP Limb)
          (:then
            (Utilities|Array|Add (Variables|Rubix|GetLeftArm) _asleft_arm_bp))
          (:CastFailed
            (bind _asright_arm_bp (Utilities|Casting|CastToRightArm_BP Limb)
              (:then
                (Utilities|Array|Add (Variables|Rubix|GetRightArm) _asright_arm_bp))
              (:CastFailed
                (bind _asleft_leg_bp (Utilities|Casting|CastToLeftLeg_BP Limb)
                  (:then
                    (Utilities|Array|Add (Variables|Rubix|GetLeftLeg) _asleft_leg_bp))
                  (:CastFailed
                    (bind _asright_leg_bp (Utilities|Casting|CastToRightLeg_BP Limb))
                    (Utilities|Array|Add (Variables|Rubix|GetRightLeg) _asright_leg_bp)))))))))))

(fn RemovefromNonMatchingLimbArrays
  (params (Limb :type Limb%202%20Object%20Reference))
  (bind _nonmatchinglimbs (Variables|Rubix|GetNonMatchingLimbs))
  (if (Utilities|Array|ContainsItem _nonmatchinglimbs Limb)
    (Utilities|Array|RemoveItem _nonmatchinglimbs Limb)
    (Utilities|Casting|CastToHead_BP 0
      (:then
        (Utilities|Array|RemoveItem (Variables|Rubix|GetHead) 0))
      (:CastFailed
        (Utilities|Casting|CastToLeftArm_BP 0
          (:then
            (Utilities|Array|RemoveItem (Variables|Rubix|GetLeftArm) 0))
          (:CastFailed
            (Utilities|Casting|CastToRightArm_BP 0
              (:then
                (Utilities|Array|RemoveItem (Variables|Rubix|GetRightArm) 0))
              (:CastFailed
                (Utilities|Casting|CastToLeftLeg_BP 0
                  (:then
                    (Utilities|Array|RemoveItem (Variables|Rubix|GetLeftLeg) 0))
                  (:CastFailed
                    (Utilities|Casting|CastToRightLeg_BP 0)
                    (Utilities|Array|RemoveItem (Variables|Rubix|GetRightLeg) 0)))))))))))

(fn GetSafestRespawnPoint
  (Utilities|Array|Clear (LocalVariables|GetDistances))
  (Utilities|Array|Clear (LocalVariables|GetSafestRespawns))
  (bind _outactors (Actor|GetAllActorsOfClass "/Script/Engine.PlayerStart"))
  (for (_array_element _array_index) _outactors
    (Utilities|Array|Add (LocalVariables|GetDistances) 1e+05)
    (Utilities|Array|Add (LocalVariables|GetSafestRespawns) (Transformation|GetActorTransform _array_element))
    (bind _outactors_2 (Actor|GetAllActorsOfClass "/Game/SkeletonWar/Blueprints/PlayerCharacters/Skele_BP.Skele_BP_C"))
    (if (<= (Utilities|Array|Length _outactors_2) 1)
      ;[1 1 1] Just choose a random spawn if there's only one player on the map
      (LocalVariables|SetSafestRespawn (Transformation|GetActorTransform (Utilities|Array|Get(acopy) _outactors (Math|Random|RandomInteger (Utilities|Array|Length _outactors)))))
      (return (LocalVariables|GetSafestRespawn))
      (else
        (for _array_element_2 _outactors_2
          (if (< (Transformation|GetDistanceTo _array_element _array_element_2) (Utilities|Array|Get(acopy) (LocalVariables|GetDistances) _array_index))
            (Utilities|Array|SetArrayElem (LocalVariables|GetDistances) _array_index (Transformation|GetDistanceTo _array_element _array_element_2)))))))
  (LocalVariables|SetSafestRespawn (Utilities|Array|Get(acopy) (LocalVariables|GetSafestRespawns) (.IndexOfMaxValue (Math|Float|MaxOfFloatArray (LocalVariables|GetDistances)))))
  (return (LocalVariables|GetSafestRespawn)))