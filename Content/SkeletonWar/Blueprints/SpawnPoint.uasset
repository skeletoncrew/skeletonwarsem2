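; SpawnPoint is a coffin bomb pickup in SkeletonWar that tops up a skeleton's bomb count on overlap, either directly or through one of its attached limbs.
; The InUse RepNotify toggles the light and plays the coffin open, paused with the lid up, or reverses it once bombs are taken.
; After pickup, a respawn timer leads to activating a random other unused spawn point, rotating bombs around the level.
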(event Custom|PauseAnim
  ;[1 1 1] Pause the animation once it's at the point where the lid is open
  (Utilities|FlowControl|Delay 1.2)
  (Variables|/Script/Engine.SkeletalMeshComponent|SetbPauseAnims (Variables|Default|GetSkeletalMesh) true)
  ;[1 1 1] If the bombs have been taken before the delay ends, unpause the anim straight away
  (if (not (Variables|Default|GetInUse))
    (CallFunction|UnpauseAnim)))

(event Custom|UnpauseAnim
  (bind _skeletalmesh (Variables|Default|GetSkeletalMesh))
  ;[1 1 1] Play the animation in reverse once the bombs have been taken
  (Components|Timeline|SetPlayRate _skeletalmesh -1.0)
  (Variables|/Script/Engine.SkeletalMeshComponent|SetbPauseAnims _skeletalmesh false))

(event Custom|StartBombRespawnTimer
  ;[1 1 1] Once the timer finishes, find the next spawn point
  (Utilities|Time|SetTimerbyEvent (EventDispatchers|CreateEvent self :!event FindSpawnandSetinUse) (Variables|Default|GetRespawnDelay)))

(event EventBeginPlay
  (if (Variables|Default|GetInitialSpawn)
    (Variables|Default|SetInUse true)))

(event Collision|EventActorBeginOverlap
  (params (OtherActor :type Actor%20Object%20Reference))
  (bind _numbombs (Variables|Default|GetNumBombs))
  (if (Variables|Default|GetInUse)
    (bind _asskele_bp (Utilities|Casting|CastToSkele_BP OtherActor)
      (:then
        (if (< (Variables|/Game/SkeletonWar/Blueprints/PlayerCharacters/Skele_BP.Skele_BP_C|GetNumberOfBombs _asskele_bp) (Variables|Default|GetNumBombs))
          (Variables|/Game/SkeletonWar/Blueprints/PlayerCharacters/Skele_BP.Skele_BP_C|SetNumberOfBombs _asskele_bp _numbombs)
          (Variables|Default|SetInUse false :!label _label)))
      (:CastFailed
        (bind _aslimb (Utilities|Casting|CastToLimb OtherActor))
        (Utilities|IsValid _aslimb
          (:Is%20Valid
            (if (and (< (Variables|/Game/SkeletonWar/Blueprints/PlayerCharacters/Skele_BP.Skele_BP_C|GetNumberOfBombs (Variables|/Game/SkeletonWar/Blueprints/Limbs/Limb.Limb_C|GetLimbParentPlayer _aslimb)) (Variables|Default|GetNumBombs)) (Variables|/Game/SkeletonWar/Blueprints/Limbs/Limb.Limb_C|GetIsAttached _aslimb))
              (Variables|/Game/SkeletonWar/Blueprints/PlayerCharacters/Skele_BP.Skele_BP_C|SetNumberOfBombs (Variables|/Game/SkeletonWar/Blueprints/Limbs/Limb.Limb_C|GetLimbParentPlayer _aslimb) _numbombs)
              (goto _label))))))))

(fn ConstructionScript)

(fn OnRepinUse
  (bind _inuse (Variables|Default|GetInUse))
  (Rendering|SetVisibility (Variables|Default|GetPointLight) _inuse false)
  (if _inuse
    (Components|Animation|PlayAnimation (Variables|Default|GetSkeletalMesh) "/Game/SkeletonWar/SkeletalMeshes/Environment/Coffin/Coffin_Export_Anim.Coffin_Export_Anim" false)
    (CallFunction|PauseAnim)
    (else
      (CallFunction|StartBombRespawnTimer)
      (CallFunction|UnpauseAnim))))

(fn FindSpawnandSetinUse
  (bind _outactors (Actor|GetAllActorsOfClass "SpawnPoint_C"))
  (if (> (Utilities|Array|Length _outactors) 1)
    (for _array_element _outactors
      (if (Variables|SpawnPoint_C|GetInUse _array_element)
        (Utilities|Array|RemoveItem _outactors _array_element)))
    (Utilities|Array|RemoveItem _outactors self))
  (Variables|SpawnPoint_C|SetInUse (Utilities|Array|Get(acopy) _outactors (Math|Random|RandomInteger (Utilities|Array|Length _outactors))) true))