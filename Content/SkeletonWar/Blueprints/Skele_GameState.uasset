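; Game state for Skeleton War that runs the round timer, scoreboard refresh and limb-loss combat log.
; On tick, the server announces the round summary through the game instance when time is up, then optionally ServerTravels to the current map after a delay.
; It also trims the combat log by line count and message age, using a parallel timestamp array.
; A delayed BeginPlay hack blanks the local player's overhead name.
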(event Custom|RoundSummaryNotify
  ;[1 1 1] Tell all clients to show the round summary
  (bind _asskele_game_instance (Utilities|Casting|CastToSkele_GameInstance (Game|GetGameInstance)))
  (Default|ShowRoundSummary _asskele_game_instance (Ability|HasAuthority)))

(event Custom|CheckGameTime
  (Networking|SwitchHasAuthority
    (:Authority
      (Utilities|FlowControl|Sequence
        (:then_0
          (Variables|Default|SetCurrentGameTime (Utilities|Time|GetGameTimeinSeconds))
          ;[1 1 1] Check game time elapsed
          (if (>= (Variables|Default|GetCurrentGameTime) (Variables|Default|GetGameEndTime))
            (Utilities|FlowControl|DoOnce false
              (:Completed
                (CallFunction|RoundSummaryNotify)))))
        (:then_1
          ;[1 1 1] Start the next round if the host isn't changing any settings
          (if (and (Variables|Default|GetAutoStartNextRound) (>= (Variables|Default|GetCurrentGameTime) (+ (Variables|Default|GetGameEndTime) (Variables|Default|GetNewGameDelay))))
            (Utilities|FlowControl|DoOnce false
              (:Completed
                (Development|ExecuteConsoleCommand (Utilities|String|Append "ServerTravel " (Class|SkeleUtilityFunctionLibrary|GetCurrentMapReference (Game|Player|GetPlayerPawn 0))))))))))))

(event Custom|UpdateCombatLog
  (params (AttackingPlayer :type Actor%20Object%20Reference) (HitPlayer :type Actor%20Object%20Reference) (Limb :type String))
  ;[1 1 1] Update the combat log when a limb is lost
  (bind _asskele_bp (Utilities|Casting|CastToSkele_BP AttackingPlayer))
  (bind _asskele_player_state (Utilities|Casting|CastToSkele_PlayerState (Variables|/Script/Engine.Pawn|GetPlayerState _asskele_bp)))
  (bind _asskele_bp_2 (Utilities|Casting|CastToSkele_BP HitPlayer))
  (bind _asskele_player_state_2 (Utilities|Casting|CastToSkele_PlayerState (Variables|/Script/Engine.Pawn|GetPlayerState _asskele_bp_2)))
  (bind _output_get (Variables|Default|SetBombVictimName (Variables|/Game/SkeletonWar/Blueprints/Skele_PlayerState.Skele_PlayerState_C|GetCurrentPlayerName _asskele_player_state_2)))
  (CallFunction|AddtoCombatLog (Utilities|String|Append (Utilities|BuildString(String) (Variables|/Game/SkeletonWar/Blueprints/Skele_PlayerState.Skele_PlayerState_C|GetCurrentPlayerName _asskele_player_state) " chopped off " _output_get "'s ") Limb)))

(event Custom|RemoveOldCombatLogMessages
  (bind _combatlog (Variables|Default|GetCombatLog))
  (bind _returnvalue (Utilities|Array|Length _combatlog))
  ;[1 1 1] Limit the number of messages shown in the combat log
  (Networking|SwitchHasAuthority
    (:Authority
      (if (> _returnvalue 0)
        (if (> _returnvalue (Variables|Default|GetMaxCombatLogLines))
          (Utilities|Array|RemoveIndex (Variables|Default|GetCombatLog) :!label _label)
          (Utilities|Array|RemoveIndex (Variables|Default|GetCombatLogTimes))
          (elif (>= (Utilities|Time|GetGameTimeinSeconds) (+ (Utilities|Array|Get(acopy) (Variables|Default|GetCombatLogTimes)) (Variables|Default|GetCombatLogMessageTime)))
            (goto _label)))))))

(event Custom|UpdateScoreboard
  ;[1 1 1] Calls the HUD's UpdateScoreboard function - this function should be called whenever a player's score changes
  (bind _asskele_player_controller (Utilities|Casting|CastToSkele_PlayerController (Game|GetPlayerController 0)))
  (Utilities|IsValid (Variables|/Game/SkeletonWar/Blueprints/Skele_PlayerController.Skele_PlayerController_C|GetSkeleHUD _asskele_player_controller)
    (:Is%20Valid
      (bind _asskele_hud (Utilities|Casting|CastToSkele_HUD (Variables|/Game/SkeletonWar/Blueprints/Skele_PlayerController.Skele_PlayerController_C|GetSkeleHUD _asskele_player_controller)))
      (Default|UpdateScoreboard _asskele_hud))))

(event EventBeginPlay
  ;[1 1 1] Hackish solution to remove the player's own name until we implement respawning
  (Utilities|FlowControl|Delay 1.0)
  (bind _asskele_bp (Utilities|Casting|CastToSkele_BP (Game|GetPlayerCharacter 0)))
  (Rendering|Components|TextRender|SetText (Variables|/Game/SkeletonWar/Blueprints/PlayerCharacters/Skele_BP.Skele_BP_C|GetOverheadText _asskele_bp) (Variables|Default|GetBlankText)))

(event EventTick
  (params (DeltaSeconds :type Float%20%28single-precision%29))
  (CallFunction|CheckGameTime)
  (CallFunction|RemoveOldCombatLogMessages))

(fn ConstructionScript)

(fn AddtoCombatLog
  (params (Message :type String))
  (Utilities|Array|Add (Variables|Default|GetCombatLog) Message)
  (Utilities|Array|Add (Variables|Default|GetCombatLogTimes) (Utilities|Time|GetGameTimeinSeconds)))