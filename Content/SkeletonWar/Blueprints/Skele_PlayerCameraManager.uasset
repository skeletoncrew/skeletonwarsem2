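; Player camera manager for the Skele character, handling lost-head vision and the view while dead or without a pawn.
; Tick watches the head entry in player 0's limb array and, on change, toggles ImpairedVision through a client event.
; BlueprintUpdateCamera overrides the view when the target is dead or not a Skele, using the level's first CameraActor or a hardcoded fallback transform.
; That fixed view allows clamped mouse look; the reverb effect code is disconnected.
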(event Custom|ClientApplyLostHeadEffect
  (params (HasHead :type Boolean))
  ;[1 1 1] Apply the lost head effect
  (CallFunction|ApplyLostHeadEffect HasHead))

(event EventBeginPlay
  (bind _outactors (Actor|GetAllActorsOfClass "/Script/Engine.CameraActor"))
  (Variables|Default|SetCameraRef (Utilities|Array|Get(acopy) _outactors)))

(event Collision|EventActorBeginOverlap
  (params (OtherActor :type Actor%20Object%20Reference)))

(event EventTick
  (params (DeltaSeconds :type Float%20%28single-precision%29))
  (bind _returnvalue (Game|Player|GetPlayerPawn 0))
  ;[1 1 1] Apply the lost head effect
  (Utilities|IsValid _returnvalue
    (:Is%20Valid
      (bind _asskele_bp (Utilities|Casting|CastToSkele_BP _returnvalue)
        (:then
          (if (Math|Boolean|NotEqual(Boolean) (Variables|Default|GetHasHead) (Utilities|Array|Get(acopy) (Variables|/Game/SkeletonWar/Blueprints/PlayerCharacters/Skele_BP.Skele_BP_C|GetHasLimb _asskele_bp)))
            (bind _output_get (Variables|Default|SetHasHead (Utilities|Array|Get(acopy) (Variables|/Game/SkeletonWar/Blueprints/PlayerCharacters/Skele_BP.Skele_BP_C|GetHasLimb _asskele_bp))))
            (CallFunction|ClientApplyLostHeadEffect _output_get)
            (else
              (Variables|Default|SetHasHead (Utilities|Array|Get(acopy) (Variables|/Game/SkeletonWar/Blueprints/PlayerCharacters/Skele_BP.Skele_BP_C|GetHasLimb _asskele_bp))))))
        (:CastFailed
          (if (Math|Boolean|NotEqual(Boolean) (Variables|Default|GetHasHead) true) :!label _label
            (Variables|Default|SetHasHead true)
            (CallFunction|ClientApplyLostHeadEffect true)
            (else
              (Variables|Default|SetHasHead true))))))
    (:Is%20Not%20Valid
      (goto _label))))

(fn ConstructionScript)

(fn BlueprintUpdateCamera
  (params (CameraTarget :type Actor%20Object%20Reference))
  (bind _returnvalue (Game|Player|GetOwningPlayerController))
  (bind _cameraref (Variables|Default|GetCameraRef))
  (bind (_deltax _deltay) (Class|PlayerController|GetInputMouseDelta _returnvalue))
  (Utilities|IsValid _cameraref
    (:Is%20Valid
      (LocalVariables|SetCameraTransform (Transformation|GetActorTransform _cameraref)))
    (:Is%20Not%20Valid
      (LocalVariables|SetCameraTransform (Math|Transform|MakeTransform "1190.846558,6274.334961,1555.493164" "-18.128296,-122.879829,0.000000"))))
  (Utilities|IsValid CameraTarget
    (:Is%20Valid
      (bind _asskele_bp (Utilities|Casting|CastToSkele_BP CameraTarget)
        (:then
          (LocalVariables|SetOverrideCamera (Variables|/Game/SkeletonWar/Blueprints/PlayerCharacters/Skele_BP.Skele_BP_C|GetIsDead _asskele_bp)))
        (:CastFailed
          (LocalVariables|SetOverrideCamera true :!label _label))))
    (:Is%20Not%20Valid
      (goto _label)))
  (if (LocalVariables|GetOverrideCamera)
    (Variables|Default|SetTurn (Math|Float|ClampAngle (+ (Variables|Default|GetTurn) _deltax) -5e+01 5e+01))
    (Variables|Default|SetLookUp (Math|Float|ClampAngle (+ (Variables|Default|GetLookUp) _deltay) -4e+01 1e+02))
    (else
      (Variables|Default|SetTurn 0.0)
      (Variables|Default|SetLookUp 0.0)))
  (return (.Location (Math|Transform|BreakTransform (LocalVariables|GetCameraTransform))) (Class|KismetMathLibrary|MakeRot (+ (.Pitch (Class|KismetMathLibrary|BreakRot (.Rotation (Math|Transform|BreakTransform (LocalVariables|GetCameraTransform))))) (Variables|Default|GetLookUp)) (+ (.Yaw (Class|KismetMathLibrary|BreakRot (.Rotation (Math|Transform|BreakTransform (LocalVariables|GetCameraTransform))))) (Variables|Default|GetTurn)) (.Roll (Class|KismetMathLibrary|BreakRot (.Rotation (Math|Transform|BreakTransform (LocalVariables|GetCameraTransform)))))) 1.1e+02 (LocalVariables|GetOverrideCamera)))

(fn ApplyLostHeadEffect
  (params (HasHead :type Boolean))
  (Variables|/Script/Engine.PostProcessComponent|SetbEnabled (Variables|Default|GetImpairedVision) (not HasHead)))