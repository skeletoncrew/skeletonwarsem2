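; Bomb spawn point for SkeletonWar that spawns a batch of bombs at its transform and hands off respawning once they are gone.
; The InUse RepNotify drives it on the server: true spawns and tracks the bombs, false starts the Skele_GameState respawn timer.
; InitialSpawn activates the point at BeginPlay, and CheckBombArray clears InUse when the tracked array is empty.
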(event EventBeginPlay
  (if (Variables|Default|GetInitialSpawn)
    (Variables|Default|SetInUse true)))

(fn ConstructionScript)

(fn OnRepinUse
  (Networking|SwitchHasAuthority
    (:Authority
      (if (Variables|Default|GetInUse)
        (for _index (range 1 (Variables|Default|GetNumBombs))
          (bind _returnvalue (Game|SpawnActorfromClass (Variables|Default|GetBombClass) (Transformation|GetWorldTransform (Variables|Transformation|GetRootComponent)) false self 0))
          (Utilities|Array|Insert (Variables|Default|GetBombArray) _returnvalue)
          (Variables|/Game/SkeletonWar/Blueprints/Weapons/BombBP.BombBP_C|SetBombSpawnPoint _returnvalue self))
        (else
          (bind _asskele_game_state (Utilities|Casting|CastToSkele_GameState (Game|GetGameState)))
          (Default|StartBombRespawnTimer _asskele_game_state (Variables|Default|GetRespawnDelay) self))))))

(fn CheckBombArray
  (if (not (Utilities|ArrayNotEmpty (Variables|Default|GetBombArray)))
    (Variables|Default|SetInUse false)
    (Development|PrintString "empty")))