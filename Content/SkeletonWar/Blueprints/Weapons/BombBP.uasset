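; Fused bomb weapon for Skeleton War that blows limbs off nearby skeleton players when it detonates.
; Tick counts down the fuse on the server, then DetonateBomb fires a radial impulse and damage, spawns explosion effects and destroys the actor.
; Living skeletons in range lose both legs, or one random arm if legless, feeding Bone Collector scoring (negative for self-hits) and the combat log.
; Hard impacts play surface-specific sounds.
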(event Custom|DetonateBomb
  (bind _returnvalue (Transformation|GetWorldLocation))
  (bind _pointtally (Variables|Default|GetPointTally))
  (bind _owningplayer (Variables|Default|GetOwningPlayer))
  (Networking|SwitchHasAuthority
    (:Authority
      (Class|RadialForceComponent|FireImpulse (Variables|Default|GetRadialForce))
      (CallFunction|SpawnExplosionParticles _returnvalue)
      (Game|Damage|ApplyRadialDamage 1e+01 _returnvalue (Variables|Default|GetBombDamageRange) 0 0 0 0 true "ECC_Visibility") ; Do damage to destructible objects
      (bind _outactors (Actor|GetAllActorsOfClass "/Game/SkeletonWar/Blueprints/PlayerCharacters/Skele_BP.Skele_BP_C"))
      (for _array_element _outactors
        (if (not (Variables|/Game/SkeletonWar/Blueprints/PlayerCharacters/Skele_BP.Skele_BP_C|GetIsDead _array_element))
          (if (<= (Transformation|GetDistanceTo _array_element) (Variables|Default|GetBombDamageRange))
            (if (> (Default|GetNumLegsAttached _array_element) 0)
              ;[1 1 1] Blow off legs if present
              (Utilities|FlowControl|Sequence
                (:then_0
                  (Utilities|IsValid (Utilities|Array|Get(acopy) (Variables|/Game/SkeletonWar/Blueprints/PlayerCharacters/Skele_BP.Skele_BP_C|GetLimbs _array_element) 3)
                    (:Is%20Valid
                      (Default|DetachLimbs (Utilities|Array|Get(acopy) (Variables|/Game/SkeletonWar/Blueprints/PlayerCharacters/Skele_BP.Skele_BP_C|GetLimbs _array_element) 3))
                      (CallFunction|ScoreLeg))))
                (:then_1
                  (Utilities|IsValid (Utilities|Array|Get(acopy) (Variables|/Game/SkeletonWar/Blueprints/PlayerCharacters/Skele_BP.Skele_BP_C|GetLimbs _array_element) 4)
                    (:Is%20Valid
                      (Default|DetachLimbs (Utilities|Array|Get(acopy) (Variables|/Game/SkeletonWar/Blueprints/PlayerCharacters/Skele_BP.Skele_BP_C|GetLimbs _array_element) 4))
                      (CallFunction|ScoreLeg))))
                (:then_2
                  ;[1 1 1] Modify scores
                  (bind _asskele_player_state (Utilities|Casting|CastToSkele_PlayerState (Variables|/Script/Engine.Pawn|GetPlayerState _owningplayer) :!label _label))
                  ;[1 0.2115 0.4145] Only modify scores if game mode is bone collector
                  (bind _is_bone_collector_ (CallFunction|GetGameMode (Game|GetGameMode)))
                  (if _is_bone_collector_
                    (if (!= _array_element _owningplayer) ; Is this another player?
                      (Default|ModifyPlayerScore _asskele_player_state _pointtally)
                      (else
                        (Default|ModifyPlayerScore _asskele_player_state (* _pointtally -1)))))
                  ;[1 1 1] Generate a hit message
                  (bind _asskele_player_state_2 (Utilities|Casting|CastToSkele_PlayerState (Variables|/Script/Engine.Pawn|GetPlayerState _array_element)))
                  (if (!= _array_element _owningplayer) ; Is this another player?
                    (Variables|Default|SetBombVictimName (Variables|/Game/SkeletonWar/Blueprints/Skele_PlayerState.Skele_PlayerState_C|GetCurrentPlayerName _asskele_player_state_2))
                    (else
                      (Variables|Default|SetBombVictimName "themself")))
                  (bind _asskele_game_state (Utilities|Casting|CastToSkele_GameState (Game|GetGameState)))
                  (Default|AddtoCombatLog _asskele_game_state (Utilities|String|Append (Utilities|String|Append (Utilities|String|Append (Variables|/Game/SkeletonWar/Blueprints/Skele_PlayerState.Skele_PlayerState_C|GetCurrentPlayerName _asskele_player_state) " blew ") (Variables|Default|GetBombVictimName)) " apart"))))
              (else
                ;[1 1 1] Randomly detach one arm
                (if (Math|Random|RandomBool)
                  (Utilities|IsValid (Utilities|Array|Get(acopy) (Variables|/Game/SkeletonWar/Blueprints/PlayerCharacters/Skele_BP.Skele_BP_C|GetLimbs _array_element) 1)
                    (:Is%20Valid
                      (Default|DetachLimbs (Utilities|Array|Get(acopy) (Variables|/Game/SkeletonWar/Blueprints/PlayerCharacters/Skele_BP.Skele_BP_C|GetLimbs _array_element) 1))
                      (CallFunction|ScoreArm)
                      (goto _label))
                    (:Is%20Not%20Valid
                      (Utilities|IsValid (Utilities|Array|Get(acopy) (Variables|/Game/SkeletonWar/Blueprints/PlayerCharacters/Skele_BP.Skele_BP_C|GetLimbs _array_element) 2)
                        (:Is%20Valid
                          (Default|DetachLimbs (Utilities|Array|Get(acopy) (Variables|/Game/SkeletonWar/Blueprints/PlayerCharacters/Skele_BP.Skele_BP_C|GetLimbs _array_element) 2))
                          (CallFunction|ScoreArm)
                          (goto _label))
                        (:Is%20Not%20Valid
                          (goto _label)))))
                  (else
                    (Utilities|IsValid (Utilities|Array|Get(acopy) (Variables|/Game/SkeletonWar/Blueprints/PlayerCharacters/Skele_BP.Skele_BP_C|GetLimbs _array_element) 2)
                      (:Is%20Valid
                        (Default|DetachLimbs (Utilities|Array|Get(acopy) (Variables|/Game/SkeletonWar/Blueprints/PlayerCharacters/Skele_BP.Skele_BP_C|GetLimbs _array_element) 2))
                        (CallFunction|ScoreArm)
                        (goto _label))
                      (:Is%20Not%20Valid
                        (Utilities|IsValid (Utilities|Array|Get(acopy) (Variables|/Game/SkeletonWar/Blueprints/PlayerCharacters/Skele_BP.Skele_BP_C|GetLimbs _array_element) 1)
                          (:Is%20Valid
                            (Default|DetachLimbs (Utilities|Array|Get(acopy) (Variables|/Game/SkeletonWar/Blueprints/PlayerCharacters/Skele_BP.Skele_BP_C|GetLimbs _array_element) 1))
                            (CallFunction|ScoreArm)
                            (goto _label))
                          (:Is%20Not%20Valid
                            (goto _label))))))))))))
      (Actor|DestroyActor))))

(event Custom|SpawnExplosionParticles
  (params (SpawnPos :type Vector :default "0, 0, 0"))
  (bind _returnvalue (Effects|SpawnEmitteratLocation "/Game/SkeletonWar/Particles/P_Explosion.P_Explosion" SpawnPos))
  (Transformation|SetRelativeScale3D _returnvalue (Variables|Default|GetExplosionScale))
  (Audio|PlaySoundatLocation (CallFunction|GetExplosionSound) SpawnPos 1.0 1.0 0.0))

(event EventBeginPlay
  (Class|GameplayStatics|PlaySoundAttached "/Game/SkeletonWar/Sounds/BombCollision/BombFuseCue.BombFuseCue" (Variables|Default|GetScene) "None" "0, 0, 0" "KeepRelativeOffset" true))

(event Collision|EventActorBeginOverlap
  (params (OtherActor :type Actor%20Object%20Reference)))

(event EventTick
  (params (DeltaSeconds :type Float%20%28single-precision%29))
  (Networking|SwitchHasAuthority
    (:Authority
      (bind _output_get (Variables|Default|SetTimeLive (+ (Variables|Default|GetTimeLive) DeltaSeconds)))
      (if (>= _output_get (Variables|Default|GetFuseTimer))
        (Utilities|FlowControl|DoOnce false
          (:Completed
            (CallFunction|DetonateBomb)))))))

(event Collision|EventHit
  (params (MyComp :type Primitive%20Component%20Object%20Reference) (Other :type Actor%20Object%20Reference) (OtherComp :type Primitive%20Component%20Object%20Reference) (bSelfMoved :type Boolean) (HitLocation :type Vector) (HitNormal :type Vector :default "0, 0, 0") (NormalImpulse :type Vector) (Hit :type Hit%20Result%20Structure%20%28by%20ref%29))
  (bind _returnvalue (Math|Vector|VectorLengthSquared NormalImpulse))
  (if (>= _returnvalue (Variables|Default|GetImpulseThreshold))
    (Audio|PlaySoundatLocation (Utilities|Select :Index (Collision|GetSurfaceType Hit) :SurfaceType_Default "/Game/SkeletonWar/Sounds/BombCollision/BombHitGrassCue.BombHitGrassCue" :SurfaceType1 "/Game/SkeletonWar/Sounds/BombCollision/BombHitGrassCue.BombHitGrassCue" :SurfaceType2 "/Game/SkeletonWar/Sounds/BombCollision/BombHitStoneCue.BombHitStoneCue" :SurfaceType3 "/Game/SkeletonWar/Sounds/BombCollision/BombHitWoodCue.BombHitWoodCue" :SurfaceType4 "/Game/SkeletonWar/Sounds/BombCollision/BombHitGlassCue.BombHitGlassCue" :SurfaceType5 "/Game/SkeletonWar/Sounds/BombCollision/BombHitMetalCue.BombHitMetalCue") HitLocation (Utilities|GetCollisionVolume _returnvalue))))

(fn ConstructionScript)

(fn ScoreLeg
  (Variables|Default|SetPointTally (+ (Variables|Default|GetPointTally) (CallFunction|GetPointsforLeg))))

(fn ScoreArm
  (Variables|Default|SetPointTally (+ (Variables|Default|GetPointTally) (CallFunction|GetPointsforArm))))