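; Replicated weapon actor for SkeletonWar that skeleton players pick up by touch and use to knock off opponents' limbs.
; Overlaps route to a server event: unequipped weapons take the first free eligible limb, while equipped, attacking weapons resolve hits.
; Enemy limb hits detach it, apply impulse, award score and update the combat log; hits and weapon clashes end the attack.
; IsWeaponEquipped's RepNotify toggles physics and socket attachment.
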(event Custom|WeaponAttackEvent
  (params (OtherActor :type Actor%20Object%20Reference))
  (bind _weaponparentplayer (Variables|Default|GetWeaponParentPlayer))
  ;[1 1 1] Call functions based on what the equipped weapon collided with
  (Utilities|Casting|CastToWeapon OtherActor
    (:then
      (CallFunction|EndAttack))
    (:CastFailed
      (bind _aslimb (Utilities|Casting|CastToLimb OtherActor))
      (if (!= (Variables|/Game/SkeletonWar/Blueprints/Limbs/Limb.Limb_C|GetLimbParentPlayer _aslimb) (Variables|Default|GetWeaponParentPlayer))
        (Default|DetachLimbs _aslimb)
        (Default|LimbApplyImpulse _aslimb)
        (CallFunction|EndAttack)
        ;;[1 1 1] Get the player and game states to update the player score and the combat log
        (bind _asskele_player_state (Utilities|Casting|CastToSkele_PlayerState (Variables|/Script/Engine.Pawn|GetPlayerState _weaponparentplayer)))
        (Default|ModifyPlayerScore _asskele_player_state (Variables|/Game/SkeletonWar/Blueprints/Limbs/Limb.Limb_C|GetLimbPointValue _aslimb))
        (bind _asskele_game_state (Utilities|Casting|CastToSkele_GameState (Game|GetGameState)))
        (Default|UpdateCombatLog _asskele_game_state _weaponparentplayer (Variables|/Game/SkeletonWar/Blueprints/Limbs/Limb.Limb_C|GetLimbParentPlayer _aslimb) (Utilities|GetDisplayName _aslimb))))))

(event Custom|GetWeaponSocketEvent
  (params (Other%20Actor :type Actor%20Object%20Reference))
  ;[1 1 1] Cycles through limbs on player to see which can equip a weapon and equips to the first available slot
  (bind _asskele_bp (Utilities|Casting|CastToSkele_BP Other%20Actor))
  (if (not (Variables|/Game/SkeletonWar/Blueprints/PlayerCharacters/Skele_BP.Skele_BP_C|GetPlayerHasWeapon _asskele_bp))
    (bind _array_element (Utilities|Array|ForEachLoopwithBreak (Variables|/Game/SkeletonWar/Blueprints/PlayerCharacters/Skele_BP.Skele_BP_C|GetLimbs _asskele_bp) :!label _label)
      (:LoopBody
        (if (Variables|/Game/SkeletonWar/Blueprints/Limbs/Limb.Limb_C|GetLimbCanEquipWeapon _array_element)
          (if (not (Variables|/Game/SkeletonWar/Blueprints/Limbs/Limb.Limb_C|GetLimbHasWeapon _array_element))
            (CallFunction|WeaponEquipEvent _array_element)
            (goto _label Break)))))))

(event Custom|WeaponEquipEvent
  (params (Limb :type Limb%20Object%20Reference))
  ;[1 1 1] Event to set variables
  (bind _output_get (Variables|Default|SetWeaponParentLimb Limb))
  (Default|SetLimbVariablesonWeaponEquip _output_get self)
  (Variables|Default|SetWeaponParentPlayer (Variables|/Game/SkeletonWar/Blueprints/Limbs/Limb.Limb_C|GetLimbParentPlayer _output_get))
  (Variables|Default|SetIsWeaponEquipped true)
  (Networking|SwitchHasAuthority
    (:Authority
      (CallFunction|WeaponPickupSound))))

(event Custom|WeaponPickupSound
  ;[1 1 1] Play a sound when equipping a weapon
  (Audio|PlaySoundatLocation "/Game/SkeletonWar/Sounds/sword_sheath_Cue.sword_sheath_Cue" (Transformation|GetWorldLocation)))

(event Custom|ServerHandleWeaponOverlap
  (params (Other%20Actor :type Actor%20Object%20Reference))
  ;[1 1 1] Call events based on whether the Weapon is equipped and attacking
  (if (Variables|Default|GetIsWeaponEquipped)
    (if (Variables|/Game/SkeletonWar/Blueprints/PlayerCharacters/Skele_BP.Skele_BP_C|GetIsPlayerAttacking (Variables|Default|GetWeaponParentPlayer))
      (CallFunction|WeaponAttackEvent Other%20Actor))
    (else
      (CallFunction|GetWeaponSocketEvent Other%20Actor))))

(event Collision|EventActorBeginOverlap
  (params (OtherActor :type Actor%20Object%20Reference))
  ;[1 1 1] On overlap call event on server
  (CallFunction|ServerHandleWeaponOverlap OtherActor))

(fn ConstructionScript
  (Variables|Default|SetIsWeaponEquipped false))

(fn OnRepIsWeaponEquipped
  (bind _isweaponequipped (Variables|Default|GetIsWeaponEquipped))
  (Physics|SetSimulatePhysics (not _isweaponequipped))
  (if _isweaponequipped
    (Class|Actor|AttachRootComponentto (Variables|/Game/SkeletonWar/Blueprints/Limbs/Limb.Limb_C|GetSkeletalMesh (Variables|Default|GetWeaponParentLimb)) (Variables|Default|GetPreferredSocket) "SnapToTarget" true)
    (else
      (Class|SceneComponent|DetachfromParent true true))))

(fn EndAttack
  (Variables|/Game/SkeletonWar/Blueprints/PlayerCharacters/Skele_BP.Skele_BP_C|SetIsPlayerAttacking (Variables|Default|GetWeaponParentPlayer) false))