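; Shovel weapon for SkeletonWar, set up as a non-limb item that prefers the SwordHand socket.
; The construction script runs the parent's, then sets weapon and limb classification and applies the shovel's physics asset to the skeletal mesh.
; On hits whose squared impulse reaches a threshold, it plays a sword impact cue chosen by surface type, with glass sharing the stone sound.
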(event Collision|EventHit
  (params (MyComp :type Primitive%20Component%20Object%20Reference) (Other :type Actor%20Object%20Reference) (OtherComp :type Primitive%20Component%20Object%20Reference) (bSelfMoved :type Boolean) (HitLocation :type Vector) (HitNormal :type Vector :default "0, 0, 0") (NormalImpulse :type Vector) (Hit :type Hit%20Result%20Structure%20%28by%20ref%29))
  (if (>= (Math|Vector|VectorLengthSquared NormalImpulse) (Variables|Default|GetImpulseTheshold))
    (Audio|PlaySoundatLocation (Utilities|Select :Index (Collision|GetSurfaceType Hit) :SurfaceType_Default "/Game/SkeletonWar/Sounds/SwordCollision/SwordHitGrassCue.SwordHitGrassCue" :SurfaceType1 "/Game/SkeletonWar/Sounds/SwordCollision/SwordHitGrassCue.SwordHitGrassCue" :SurfaceType2 "/Game/SkeletonWar/Sounds/SwordCollision/SwordHitStoneCue.SwordHitStoneCue" :SurfaceType3 "/Game/SkeletonWar/Sounds/SwordCollision/SwordHitWoodCue.SwordHitWoodCue" :SurfaceType4 "/Game/SkeletonWar/Sounds/SwordCollision/SwordHitStoneCue.SwordHitStoneCue" :SurfaceType5 "/Game/SkeletonWar/Sounds/SwordCollision/SwordHitMetalCue.SwordHitMetalCue") HitLocation)))

(event EventBeginPlay)

(event Collision|EventActorBeginOverlap
  (params (OtherActor :type Actor%20Object%20Reference))
  (|CallParentFunction 0))

(fn ConstructionScript
  (|CallParentFunction)
  (Variables|Default|SetIsLimb false)
  (Variables|Default|SetIsWeapon true)
  (Variables|Default|SetDefaultType "Weapon")
  (Variables|Default|SetPreferredSocket "SwordHand")
  (Variables|Default|SetDefaultLimbType "NewEnumerator1")
  (Components|SkinnedMesh|SetPhysicsAsset (Variables|Default|GetSkeletalMesh) "/Game/SkeletonWar/SkeletalMeshes/Weapons/Sword/Shovel_Export_Physics.Shovel_Export_Physics" true)
  (Variables|Default|SetWeaponType "NewEnumerator2"))