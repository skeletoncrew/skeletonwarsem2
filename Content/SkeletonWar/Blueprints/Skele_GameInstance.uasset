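; Game instance for Skeleton War that manages menu flow, hosting and joining games, and saved player settings.
; A ChangeState macro acts as a state machine, removing the outgoing widget and destroying the session when leaving gameplay for non-overlay screens.
; Show events lazily create and cache their widgets, while session, network and travel failures feed a shared error dialog.
; Startup applies saved options or prompts for a player name with a random default.
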(event Custom|ShowHowToPlay
  (params (Ingame :type Boolean))
  (bind _returnvalue (Game|GetPlayerController 0))
  ;[1 1 1] Show the rewards chest screen
  (Utilities|ChangeState "NewEnumerator11"
    (:NewState
      (Utilities|IsValid (Variables|Default|GetRewardsChest)
        (:Is%20Valid
          _)
        (:Is%20Not%20Valid
          (bind _returnvalue_2 (UserInterface|CreateWidget "/Game/SkeletonWar/UMG/RewardsChest.RewardsChest_C" _returnvalue))
          (Variables|Default|SetRewardsChest _returnvalue_2)))
      (Default|SetMainBackground (Variables|Default|GetRewardsChest) Ingame)
      (UserInterface|Viewport|AddtoViewport (Variables|Default|GetRewardsChest) 1)
      (Input|SetInputModeUIOnly _returnvalue (Variables|Default|GetRewardsChest) false))))

(event Custom|ShowOptionsMenu
  (params (Ingame :type Boolean))
  (bind _returnvalue (Game|GetPlayerController 0))
  ;[1 1 1] Show the options menu
  (Utilities|ChangeState "NewEnumerator4"
    (:NewState
      (Utilities|IsValid (Variables|Default|GetOptionsMenu)
        (:Is%20Valid
          _)
        (:Is%20Not%20Valid
          (bind _returnvalue_2 (UserInterface|CreateWidget "/Game/SkeletonWar/UMG/OptionsMenu.OptionsMenu_C" _returnvalue))
          (Variables|Default|SetOptionsMenu _returnvalue_2)))
      (Default|SetMainBackground (Variables|Default|GetOptionsMenu) Ingame)
      (UserInterface|Viewport|AddtoViewport (Variables|Default|GetOptionsMenu) 1)
      (Input|SetInputModeUIOnly _returnvalue (Variables|Default|GetOptionsMenu) false))))

(event Custom|DestroySession
  ;[1 1 1] Destroy the session
  (|DestroySession (Game|GetPlayerController 0)))

(event Custom|ShowMainMenu
  (bind _returnvalue (Game|GetPlayerController 0))
  ;[1 1 1] Show the main menu
  (Utilities|ChangeState "NewEnumerator1"
    (:NewState
      (Utilities|IsValid (Variables|Default|GetMainMenu)
        (:Is%20Valid
          _)
        (:Is%20Not%20Valid
          (bind _returnvalue_2 (UserInterface|CreateWidget "/Game/SkeletonWar/UMG/MainMenu.MainMenu_C" _returnvalue))
          (Variables|Default|SetMainMenu _returnvalue_2)))
      (UserInterface|Viewport|AddtoViewport (Variables|Default|GetMainMenu) 0)
      (Input|SetInputModeUIOnly _returnvalue (Variables|Default|GetMainMenu) false)
      (Variables|/Script/Engine.PlayerController|SetbShowMouseCursor _returnvalue true))))

(event Custom|ShowServerList
  (bind _returnvalue (Game|GetPlayerController 0))
  ;[1 1 1] Show the server list screen
  (Utilities|ChangeState "NewEnumerator2"
    (:NewState
      (Utilities|IsValid (Variables|Default|GetServerList)
        (:Is%20Valid
          _)
        (:Is%20Not%20Valid
          (bind _returnvalue_2 (UserInterface|CreateWidget "/Game/SkeletonWar/UMG/ServerList.ServerList_C" _returnvalue))
          (bind _output_get (Variables|Default|SetServerList _returnvalue_2))
          (Variables|/Game/SkeletonWar/UMG/ServerList.ServerList_C|SetLocalIP _output_get "Not found") ; This functionality is currently unused, because apparently it's highly complicated to find your own computer's local IP in C++
        ))
      (UserInterface|Viewport|AddtoViewport (Variables|Default|GetServerList) 0)
      (Input|SetInputModeUIOnly _returnvalue (Variables|Default|GetServerList) false))))

(event Custom|JoinFromServerList
  (params (SessionResult :type Blueprint%20Session%20Result%20Structure))
  ;[1 1 1] Join a session
  (CallFunction|ShowLoadingScreen)
  (|JoinSession (Game|GetPlayerController 0) SessionResult
    (:OnFailure
      (Utilities|DisplayErrorDialog "Failed to join session."))))

(event Custom|ShowLoadingScreen
  (bind _returnvalue (Game|GetPlayerController 0))
  ;[1 1 1] Show the loading screen (when you join or host a game)
  (Utilities|ChangeState "NewEnumerator5"
    (:NewState
      (Utilities|IsValid (Variables|Default|GetLoadingScreen)
        (:Is%20Valid
          _)
        (:Is%20Not%20Valid
          (bind _returnvalue_2 (UserInterface|CreateWidget "/Game/SkeletonWar/UMG/LoadingScreen.LoadingScreen_C" _returnvalue))
          (Variables|Default|SetLoadingScreen _returnvalue_2)))
      (UserInterface|Viewport|AddtoViewport (Variables|Default|GetLoadingScreen) 0)
      (Input|SetInputModeUIOnly _returnvalue (Variables|Default|GetLoadingScreen) false))))

(event Custom|HostGame
  (params (Settings :type Server%20Settings%20Struct%20Structure) (NewSession :type Boolean))
  (bind (_servername _gamemode _maxplayers _gametime _enablelan _isdedicated) (Utilities|Struct|BreakServerSettings_Struct Settings))
  (bind _returnvalue (Game|GetPlayerController 0))
  ;[1 1 1] Host a game with the given settings
  (Variables|Default|SetServerSettings Settings)
  (CallFunction|ShowLoadingScreen)
  (if NewSession
    (|Session _returnvalue _maxplayers _enablelan
      (:OnSuccess
        (Game|OpenLevel(byName) "Abbey" true (select _isdedicated "dedicated" "listen"))
        (Input|SetInputModeGameOnly _returnvalue :!label _label))
      (:OnFailure
        (Utilities|DisplayErrorDialog "Failed to create session.")))
    (else
      (Development|ExecuteConsoleCommand "ServerTravel Abbey")
      (goto _label))))

(event Custom|JoinByDirectIP
  (params (IP%20Address :type String))
  ;[1 1 1] Join a game via a direct IP address
  (CallFunction|ShowLoadingScreen)
  (Input|SetInputModeGameOnly (Game|GetPlayerController 0))
  (Development|ExecuteConsoleCommand (Utilities|String|Append "open " IP%20Address))
  (Utilities|FlowControl|Delay 5.0)
  (if (Utilities|Enum|Equal(Enum) (Class|SkeleUtilityFunctionLibrary|GetCurrentMapReference (Game|Player|GetPlayerPawn 0)) "MainMenu_Level")
    (Utilities|DisplayErrorDialog "Failed to connect.")))

(event Custom|ShowControlsMenu
  (params (Ingame :type Boolean))
  (bind _returnvalue (Game|GetPlayerController 0))
  ;[1 1 1] Show the controls screen
  (Utilities|ChangeState "NewEnumerator12"
    (:NewState
      (Utilities|IsValid (Variables|Default|GetControlsMenu)
        (:Is%20Valid
          _)
        (:Is%20Not%20Valid
          (bind _returnvalue_2 (UserInterface|CreateWidget "/Game/SkeletonWar/UMG/Controls.Controls_C" _returnvalue))
          (Variables|Default|SetControlsMenu _returnvalue_2)))
      (Default|SetMainBackground (Variables|Default|GetControlsMenu) Ingame)
      (UserInterface|Viewport|AddtoViewport (Variables|Default|GetControlsMenu) 1)
      (Input|SetInputModeUIOnly _returnvalue (Variables|Default|GetControlsMenu) false))))

(event Custom|ShowRoundSummary
  (params (HasAuthority :type Boolean))
  (bind _returnvalue (Game|GetPlayerController 0))
  ;[1 1 1] Show the round summary widget
  (Utilities|IsValid (Variables|Default|GetRoundSummary)
    (:Is%20Valid
      _)
    (:Is%20Not%20Valid
      (bind _returnvalue_2 (UserInterface|CreateWidget "/Game/SkeletonWar/UMG/RoundSummary.RoundSummary_C" _returnvalue))
      (Variables|Default|SetRoundSummary _returnvalue_2)))
  (Widget|SetVisibility (Variables|/Game/SkeletonWar/UMG/RoundSummary.RoundSummary_C|GetChangeServerSettingsButton (Variables|Default|GetRoundSummary)) (select HasAuthority "Visible" "Collapsed"))
  (UserInterface|Viewport|AddtoViewport (Variables|Default|GetRoundSummary) 1)
  (if HasAuthority
    (Input|SetInputModeUIOnly _returnvalue (Variables|Default|GetRoundSummary) false)
    (else
      (Input|SetInputModeGameOnly _returnvalue))))

(event Custom|ShowCreditsMenu
  (bind _returnvalue (Game|GetPlayerController 0))
  ;[1 1 1] Show the credits
  (Utilities|ChangeState "NewEnumerator10"
    (:NewState
      (Utilities|IsValid (Variables|Default|GetCreditsMenu)
        (:Is%20Valid
          _)
        (:Is%20Not%20Valid
          (bind _returnvalue_2 (UserInterface|CreateWidget "/Game/SkeletonWar/UMG/CreditsMenu.CreditsMenu_C" _returnvalue))
          (Variables|Default|SetCreditsMenu _returnvalue_2)))
      (UserInterface|Viewport|AddtoViewport (Variables|Default|GetCreditsMenu) 0)
      (Input|SetInputModeUIOnly _returnvalue (Variables|Default|GetCreditsMenu) false))))

(event Custom|ShowHostMenu
  (params (Ingame :type Boolean))
  (bind _returnvalue (Game|GetPlayerController 0))
  ;[1 1 1] Show the host game menu
  (Utilities|ChangeState "NewEnumerator3"
    (:NewState
      (Utilities|IsValid (Variables|Default|GetHostMenu)
        (:Is%20Valid
          _)
        (:Is%20Not%20Valid
          (bind _returnvalue_2 (UserInterface|CreateWidget "/Game/SkeletonWar/UMG/HostMenu.HostMenu_C" _returnvalue))
          (Variables|Default|SetHostMenu _returnvalue_2)))
      (Default|SetMainBackground (Variables|Default|GetHostMenu) Ingame)
      (UserInterface|Viewport|AddtoViewport (Variables|Default|GetHostMenu) 1)
      (Input|SetInputModeUIOnly _returnvalue (Variables|Default|GetHostMenu) false))))

(event EventHandleNetworkError
  (params (FailureType :type ENetworkFailure%20Enum :default "NetDriverAlreadyExists") (bIsServer :type Boolean))
  ;[1 1 1] Handle network errors
  (if (not bIsServer)
    (Utilities|DisplayErrorDialog (CallFunction|NetworkErrortoString FailureType))))

(event EventHandleTravelError
  (params (FailureType :type ETravelFailure%20Enum :default "NoLevel"))
  ;[1 1 1] Handle travel errors
  (Utilities|DisplayErrorDialog (CallFunction|TravelErrortoString FailureType)))

(fn NetworkErrortoString
  (params (InError :type ENetworkFailure%20Enum))
  (switch Utilities|FlowControl|Switch|SwitchonENetworkFailure InError
    (:NetDriverAlreadyExists
      (LocalVariables|SetErrorString "Lost connection to host." :!label _label))
    (:NetDriverCreateFailure
      (goto _label))
    (:NetDriverListenFailure
      (goto _label))
    (:ConnectionLost
      (goto _label))
    (:ConnectionTimeout
      (LocalVariables|SetErrorString "Connection timed out."))
    (:FailureReceived
      (goto _label))
    (:OutdatedClient
      (goto _label))
    (:OutdatedServer
      (goto _label))
    (:PendingConnectionFailure
      (goto _label)))
  (return (LocalVariables|GetErrorString)))

(fn StartPlayingState
  (params (ShowCursor :type Boolean))
  (bind _returnvalue (Game|GetPlayerController 0))
  (bind _roundsummary (Variables|Default|GetRoundSummary))
  (Utilities|ChangeState "NewEnumerator7"
    (:NewState
      (if ShowCursor
        (Input|SetInputModeUIOnly _returnvalue 0 false)
        (Variables|/Script/Engine.PlayerController|SetbShowMouseCursor _returnvalue true)
        (Utilities|IsValid _roundsummary
          (:Is%20Valid
            (Class|Widget|SetUserFocus _roundsummary _returnvalue)))
        (else
          (Input|SetInputModeGameOnly _returnvalue)
          (Variables|/Script/Engine.PlayerController|SetbShowMouseCursor _returnvalue false))))))

(fn BeginPlayShowMainMenu
  (Utilities|IsCurrentState "NewEnumerator0"
    (:True
      (bind _founddata (CallFunction|CheckforSaveData))
      (if _founddata
        (CallFunction|ShowMainMenu :!label _label)))
    (:False
      (goto _label))))

(fn TravelErrortoString
  (params (InError :type ETravelFailure%20Enum))
  (return (Utilities|String|Append "Failed to travel. " (Utilities|String|EnumtoString InError))))

(fn GetState
  (return (Variables|Default|GetCurrentState)))

(fn CheckforSaveData
  (bind _returnvalue (Game|GetPlayerController 0))
  (bind _rng (Variables|Default|GetRNG))
  (bind _saveslotname (Variables|Default|GetSaveSlotName))
  (bind _returnvalue_2 (SaveGame|DoesSaveGameExist _saveslotname))
  (if _returnvalue_2
    ;[1 1 1] Apply saved options if found
    (bind _returnvalue_3 (SaveGame|LoadGamefromSlot _saveslotname))
    (bind _asskele_save_data (Utilities|Casting|CastToSkele_SaveData _returnvalue_3)
      (:then
        (Variables|Default|SetPlayerName (Variables|/Game/SkeletonWar/Blueprints/Skele_SaveData.Skele_SaveData_C|GetPlayerName _asskele_save_data))
        (CallFunction|ApplyOptions (Variables|/Game/SkeletonWar/Blueprints/Skele_SaveData.Skele_SaveData_C|GetResolution _asskele_save_data) (Variables|/Game/SkeletonWar/Blueprints/Skele_SaveData.Skele_SaveData_C|GetFullscreen _asskele_save_data) (Variables|/Game/SkeletonWar/Blueprints/Skele_SaveData.Skele_SaveData_C|GetVSync _asskele_save_data) (Variables|/Game/SkeletonWar/Blueprints/Skele_SaveData.Skele_SaveData_C|GetShadows _asskele_save_data) (Variables|/Game/SkeletonWar/Blueprints/Skele_SaveData.Skele_SaveData_C|GetMotionBlur _asskele_save_data) (Variables|/Game/SkeletonWar/Blueprints/Skele_SaveData.Skele_SaveData_C|GetTurnRateScalar _asskele_save_data) (Variables|/Game/SkeletonWar/Blueprints/Skele_SaveData.Skele_SaveData_C|GetLookUpRateScalar _asskele_save_data) (Variables|/Game/SkeletonWar/Blueprints/Skele_SaveData.Skele_SaveData_C|GetInvertYAxis _asskele_save_data) (Variables|/Game/SkeletonWar/Blueprints/Skele_SaveData.Skele_SaveData_C|GetInvertXAxis _asskele_save_data) (Variables|/Game/SkeletonWar/Blueprints/Skele_SaveData.Skele_SaveData_C|GetAmbientOcclusion _asskele_save_data) (Variables|/Game/SkeletonWar/Blueprints/Skele_SaveData.Skele_SaveData_C|GetAALevel _asskele_save_data) (Variables|/Game/SkeletonWar/Blueprints/Skele_SaveData.Skele_SaveData_C|GetViewDistance _asskele_save_data) (Variables|/Game/SkeletonWar/Blueprints/Skele_SaveData.Skele_SaveData_C|GetChunkLifetime _asskele_save_data)))
      (:CastFailed
        ;[1 1 1] Prompt the player to enter a name
        (bind _returnvalue_4 (UserInterface|CreateWidget "/Game/SkeletonWar/UMG/PlayerNameInput.PlayerNameInput_C" _returnvalue :!label _label))
        (Math|Random|SetRandomStreamSeed _rng (Math|DateTime|GetMillisecond (Math|DateTime|Now)))
        (bind _returnvalue_5 (Class|SkeleUtilityFunctionLibrary|GetDefaultPlayerNamesfromFile))
        (Default|SetPlayerNameText _returnvalue_4 (Utilities|Array|Get(acopy) _returnvalue_5 (Class|KismetMathLibrary|RandomIntegerfromStream (Utilities|Array|Length _returnvalue_5) _rng)))
        (UserInterface|Viewport|AddtoViewport _returnvalue_4 0)
        (Input|SetInputModeGameandUI _returnvalue _returnvalue_4 false false)))
    (else
      (Development|ExecuteConsoleCommand "r.SetRes 1920x1080wf" _returnvalue)
      (goto _label)))
  (return _returnvalue_2))

(fn SavePlayerName
  (params (Name :type String))
  (bind _output_get (Variables|Default|SetPlayerName Name))
  (bind _returnvalue (SaveGame|CreateSaveGameObject "/Game/SkeletonWar/Blueprints/Skele_SaveData.Skele_SaveData_C"))
  (bind _asskele_save_data (Utilities|Casting|CastToSkele_SaveData _returnvalue))
  (Variables|/Game/SkeletonWar/Blueprints/Skele_SaveData.Skele_SaveData_C|SetPlayerName _asskele_save_data _output_get)
  (SaveGame|SaveGametoSlot _asskele_save_data (Variables|Default|GetSaveSlotName)))

(fn ShowErrorMessage
  (params (Message :type String))
  (Utilities|DisplayErrorDialog Message))