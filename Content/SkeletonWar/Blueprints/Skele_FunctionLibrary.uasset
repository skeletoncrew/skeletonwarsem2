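; Skele_FunctionLibrary is SkeletonWar's shared helper library, centralising sound and music assets, per-limb point values and common gameplay checks.
; Helpers test socketed limbs for arm or leg class, compare limb and player bone colours, and flag Bone Collector or Rubix mode.
; UI helpers style gravestone and menu buttons by keyboard focus.
; ApplyOptions sets resolution, fullscreen, VSync and shadow quality through console commands.
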(fn IsArm?
  (params (LimbArray :type Array%20of%20Limb%20Object%20References) (Socket :type LimbEnum%20Enum))
  (bind _returnvalue (Math|Conversions|ToInteger(Byte) Socket))
  (bind _item (Utilities|Array|Get(acopy) LimbArray _returnvalue))
  (bind _returnvalue_2 (Utilities|GetClass _item))
  (return (or (== _returnvalue_2 "/Game/SkeletonWar/Blueprints/Limbs/LeftArm_BP.LeftArm_BP_C") (== _returnvalue_2 "/Game/SkeletonWar/Blueprints/Limbs/RightArm_BP.RightArm_BP_C"))))

(fn IsLeg?
  (params (LimbArray :type Array%20of%20Limb%20Object%20References) (LimbSocket :type LimbEnum%20Enum))
  (bind _returnvalue (Math|Conversions|ToInteger(Byte) LimbSocket))
  (bind _item (Utilities|Array|Get(acopy) LimbArray _returnvalue))
  (bind _returnvalue_2 (Utilities|GetClass _item))
  (return (or (== _returnvalue_2 "/Game/SkeletonWar/Blueprints/Limbs/LeftLeg_BP.LeftLeg_BP_C") (== _returnvalue_2 "/Game/SkeletonWar/Blueprints/Limbs/RightLeg_BP.RightLeg_BP_C"))))

(fn GetWeaponPickupSound
  (return "/Game/SkeletonWar/Sounds/sword_sheath_Cue.sword_sheath_Cue"))

(fn GetHeadDetachSound
  (return "/Game/SkeletonWar/Sounds/neck_snap_Cue.neck_snap_Cue"))

(fn GetArmDetachSound
  (return "/Game/SkeletonWar/Sounds/bone_break_Cue.bone_break_Cue"))

(fn GetLegDetachSound
  (return "/Game/SkeletonWar/Sounds/bone_break_leg_Cue.bone_break_leg_Cue"))

(fn GetLimbAttachSound
  (return "/Game/SkeletonWar/Sounds/bone_pickup_Cue.bone_pickup_Cue"))

(fn GetAttackSwooshSound
  (return "/Game/SkeletonWar/Sounds/AttackSwooshSound_Cue.AttackSwooshSound_Cue"))

(fn GetGameplayMusic
  (return "/Game/SkeletonWar/Sounds/Idle_Jazz.Idle_Jazz"))

(fn GetMainMenuMusic
  (return "/Game/SkeletonWar/Sounds/Skeletal_Jazz_v2.Skeletal_Jazz_v2"))

(fn GetLFootstepSound
  (return "/Game/SkeletonWar/Sounds/footstep_forest01_Cue.footstep_forest01_Cue"))

(fn GetRFootstepSound
  (return "/Game/SkeletonWar/Sounds/footstep_forest02_Cue.footstep_forest02_Cue"))

(fn GetExplosionSound
  (return "/Game/SkeletonWar/Sounds/Explosion_Cue.Explosion_Cue"))

(fn GetPointsforLeg
  (return 2))

(fn GetPointsforArm
  (return 1))

(fn GetPointsforHead
  (return 3))

(fn GetGravestoneButtonStyle
  (params (Hovered :type Boolean))
  (if Hovered
    (LocalVariables|SetReturnValue (LocalVariables|GetHoveredStyle))
    (else
      (LocalVariables|SetReturnValue (LocalVariables|GetNormalStyle))))
  (return (LocalVariables|GetReturnValue)))

(fn GetMenuButtonStyle
  (params (Hovered :type Boolean))
  (if Hovered
    (LocalVariables|SetReturnValue (LocalVariables|GetHoveredStyle))
    (else
      (LocalVariables|SetReturnValue (LocalVariables|GetNormalStyle))))
  (return (LocalVariables|GetReturnValue)))

(fn ApplyGravestoneButtonStyle
  (params (Button :type Button%20Object%20Reference))
  (Variables|/Script/UMG.Button|SetWidgetStyle Button (CallFunction|GetGravestoneButtonStyle (Class|Widget|HasKeyboardFocus Button))))

(fn ApplyMenuButtonStyle
  (params (Button :type Button%20Object%20Reference))
  (Variables|/Script/UMG.Button|SetWidgetStyle Button (CallFunction|GetMenuButtonStyle (Class|Widget|HasKeyboardFocus Button))))

(fn GetMenuSelectionSound
  (return "/Game/SkeletonWar/Sounds/finger_snap.finger_snap"))

(fn GetGameMode
  (params (Game%20Mode :type Game%20Mode%20Object%20Reference))
  (Utilities|IsValid Game%20Mode
    (:Is%20Valid
      (bind _asskele_game_mode (Utilities|Casting|CastToSkele_GameMode Game%20Mode))
      (return (Utilities|Enum|Equal(Enum) (Variables|/Game/SkeletonWar/Blueprints/Skele_GameMode.Skele_GameMode_C|GetGameMode _asskele_game_mode) "NewEnumerator0") (Utilities|Enum|Equal(Enum) (Variables|/Game/SkeletonWar/Blueprints/Skele_GameMode.Skele_GameMode_C|GetGameMode _asskele_game_mode) "NewEnumerator1")))))

(fn IsSameColour?
  (params (Limb :type Limb%20Object%20Reference) (Player :type Skele%20BP%20Object%20Reference))
  (return (Utilities|Name|Equal(Name) (Variables|/Game/SkeletonWar/Blueprints/Limbs/Limb.Limb_C|GetBoneColour Limb) (Variables|/Game/SkeletonWar/Blueprints/PlayerCharacters/Skele_BP.Skele_BP_C|GetBoneColour Player))))

(fn ApplyOptions
  (params (Resolution :type String) (Fullscreen :type Boolean) (VSync :type Boolean) (Shadows :type Boolean))
  (Development|ExecuteConsoleCommand 0 (Utilities|String|Append "r.setRes " (Utilities|String|Append Resolution (select Fullscreen "wf" ""))))
  (Development|ExecuteConsoleCommand 0 (Utilities|String|BuildString(Integer) "" "r.VSync " (select VSync 1 0)))
  (Development|ExecuteConsoleCommand 0 (Utilities|String|BuildString(Integer) "" "r.ShadowQuality " (select Shadows 3 0))))