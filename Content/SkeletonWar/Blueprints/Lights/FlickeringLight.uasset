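; FlickeringLight is a light Blueprint that makes a warm amber point light flicker.
; The construction script sets the color, and Tick uses a Delay of FlickerSpeed to pace changes to a random intensity between LowIntensity and HighIntensity.
; A random comparison after each change can start a second Delay, but nothing follows it, so it does not pause the flicker.
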(event EventTick
  (params (DeltaSeconds :type Float%20%28single-precision%29))
  (bind _lowintensity (Variables|Default|GetLowIntensity))
  (bind _highintensity (Variables|Default|GetHighIntensity))
  (bind _returnvalue (Math|Random|RandomFloatinRange _lowintensity _highintensity))
  (Utilities|FlowControl|Delay (Variables|Default|GetFlickerSpeed))
  (Rendering|Components|Light|SetIntensity (Variables|Default|GetPointLight) _returnvalue)
  (if (> _returnvalue (* _returnvalue 0.95))
    (Utilities|FlowControl|Delay 2.0)))

(fn ConstructionScript
  (Rendering|Components|Light|SetLightColor (Variables|Default|GetPointLight) "(R=0.835000,G=0.536554,B=0.048414,A=1.000000)"))