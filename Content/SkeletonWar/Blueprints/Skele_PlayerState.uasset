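; Skele_PlayerState is the SkeletonWar player state, holding a player's score and triggering scoreboard refreshes on Skele_GameState.
; ModifyPlayerScore adds a modifier through UpdatePlayerScore, which writes only with authority, then refreshes the scoreboard.
; On authority, BeginPlay calls an empty AssignPlayerInfo and refreshes the scoreboard.
; Disconnected logic would draw a random unique name from Skele_GameMode's pool, but it never runs.
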(event Custom|AssignPlayerInfo)

(event Custom|UpdatePlayerScore
  (params (NewScore :type Integer :default 0))
  (Networking|SwitchHasAuthority
    (:Authority
      (Variables|Default|SetPlayerScore NewScore))))

(event EventBeginPlay
  (Networking|SwitchHasAuthority
    (:Authority
      (CallFunction|AssignPlayerInfo)
      (bind _asskele_game_state (Utilities|Casting|CastToSkele_GameState (Game|GetGameState)))
      (Default|UpdateScoreboard _asskele_game_state))))

(event EventTick
  (params (DeltaSeconds :type Float%20%28single-precision%29)))

(fn ConstructionScript)

(fn ModifyPlayerScore
  (params (Modifier :type Integer :default 0))
  (CallFunction|UpdatePlayerScore (+ (Variables|Default|GetPlayerScore) Modifier))
  (bind _asskele_game_state (Utilities|Casting|CastToSkele_GameState (Game|GetGameState)))
  (Default|UpdateScoreboard _asskele_game_state))