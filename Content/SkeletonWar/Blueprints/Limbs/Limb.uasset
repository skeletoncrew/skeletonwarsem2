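; Detachable skeleton limb that players pick up on overlap and that attached legs use to knock off rival skulls.
; The server attaches it to its preferred socket, falling back to the paired socket, or to arm sockets for legs.
; An IsAttached RepNotify toggles physics and socket attachment, while detaching starts a pickup delay and releases any held weapon.
; Tick derives the animation state and blendspace from the owner's limb layout.
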(event EventTick
  (params (DeltaSeconds :type Float%20%28single-precision%29))
  (CallFunction|SetAnimationState)
  (switch Utilities|FlowControl|Switch|SwitchonAnimStateEnum (Variables|Default|GetAnimState)
    (:NewEnumerator0
      ;[0.1045 1 0] Set animation blendspace to be used
      (Variables|IdleRunBSArrays|SetCurrent_IdleRunBSpaces (Variables|IdleRunBSArrays|Get2L_IdleRunBSpaces)))
    (:NewEnumerator1
      (Variables|IdleRunBSArrays|SetCurrent_IdleRunBSpaces (Variables|IdleRunBSArrays|Get1L_IdleRunBSpaces)))
    (:NewEnumerator2
      (Variables|IdleRunBSArrays|SetCurrent_IdleRunBSpaces (Variables|IdleRunBSArrays|Get0L_IdleRunBSpaces)))
    (:NewEnumerator3
      (Variables|IdleRunBSArrays|SetCurrent_IdleRunBSpaces (Variables|IdleRunBSArrays|GetC_IdleRunBSpaces)))
    (:NewEnumerator4
      (Variables|IdleRunBSArrays|SetCurrent_IdleRunBSpaces (Variables|IdleRunBSArrays|GetAF_IdleRunBSpaces)))))

(event Collision|EventActorBeginOverlap
  (params (OtherActor :type Actor%20Object%20Reference))
  (bind _aslimb (Utilities|Casting|CastToLimb OtherActor)
    (:then
      ;[1 1 1] Let legs knock off skulls
      (if (>= (Variables|Default|GetPreferredSocketIndex) 3)
        (if (== (Variables|Limb_C|GetPreferredSocketIndex _aslimb) 0)
          (if (Variables|Limb_C|GetIsAttached _aslimb)
            (if (and (!= (Variables|Default|GetLimbParentPlayer) (Variables|Limb_C|GetLimbParentPlayer _aslimb)) (Variables|Default|GetIsAttached))
              (CallFunction|DetachLimbs _aslimb))))))
    (:CastFailed
      (bind _asskele_bp (Utilities|Casting|CastToSkele_BP OtherActor))
      (if (not (Variables|/Game/SkeletonWar/Blueprints/PlayerCharacters/Skele_BP.Skele_BP_C|GetIsDead _asskele_bp))
        (if (not (Utilities|Array|ContainsItem (Variables|/Game/SkeletonWar/Blueprints/PlayerCharacters/Skele_BP.Skele_BP_C|GetLimbs _asskele_bp) self))
          (if (not (Variables|Default|GetIsAttached))
            (CallFunction|PlayerOverlapDetection _asskele_bp)))))))

(event Custom|Detach%20Limbs
  (bind _limbparentplayer (Variables|Default|GetLimbParentPlayer))
  (bind _actualsocketindex (Variables|Default|GetActualSocketIndex))
  ;[1 1 1] Update variables to tell the server the limb's detached
  (CallFunction|SetLimbVariablesonWeaponDetach)
  (Variables|Default|SetReadyToAttach false)
  (Variables|Default|SetIsAttached false)
  (Utilities|Array|SetArrayElem (Variables|/Game/SkeletonWar/Blueprints/PlayerCharacters/Skele_BP.Skele_BP_C|GetLimbs _limbparentplayer) _actualsocketindex 0)
  (Utilities|Array|SetArrayElem (Variables|/Game/SkeletonWar/Blueprints/PlayerCharacters/Skele_BP.Skele_BP_C|GetHasLimb _limbparentplayer) _actualsocketindex false)
  (Networking|SwitchHasAuthority
    (:Authority
      (CallFunction|DetachLimbSound))
    (:Remote
      _))
  (Utilities|FlowControl|Delay (Variables|Default|GetLimbPickupDelay))
  (Variables|Default|SetReadyToAttach true)
  (Variables|Default|SetPlayerStateChanged true))

(event Custom|DetachLimbSound
  (bind _returnvalue (Transformation|GetWorldLocation))
  (bind _preferredsocketindex (Variables|Default|GetPreferredSocketIndex))
  ;[1 1 1] Play a sound when a limb is detached
  (if (== _preferredsocketindex 0)
    (Audio|PlaySoundatLocation "/Game/SkeletonWar/Sounds/neck_snap_Cue.neck_snap_Cue" _returnvalue)
    (elif (<= _preferredsocketindex 2)
      (Audio|PlaySoundatLocation "/Game/SkeletonWar/Sounds/bone_break_Cue.bone_break_Cue" _returnvalue)
      (else
        (Audio|PlaySoundatLocation "/Game/SkeletonWar/Sounds/bone_break_leg_Cue.bone_break_leg_Cue" _returnvalue)))))

(event Custom|AttachLimbSound
  ;[1 1 1] Play a sound when a limb is attached
  (Audio|PlaySoundatLocation "/Game/SkeletonWar/Sounds/bone_pickup_Cue.bone_pickup_Cue" (Transformation|GetWorldLocation)))

(event Custom|AttachLimbs
  (params (Player :type Skele%20BP%20Object%20Reference) (SocketIndex :type Integer :default 0))
  (bind _returnvalue (Math|Integer|%(Integer) SocketIndex 2))
  (bind _returnvalue_2 (Math|Integer|%(Integer) SocketIndex 2))
  (bind _haslimb (Variables|/Game/SkeletonWar/Blueprints/PlayerCharacters/Skele_BP.Skele_BP_C|GetHasLimb Player))
  (bind _returnvalue_3 (* _returnvalue 2))
  (bind _returnvalue_4 (+ _returnvalue_2 1))
  (bind _returnvalue_5 (- _returnvalue_3 1))
  (bind _returnvalue_6 (+ _returnvalue_4 1))
  (bind _returnvalue_7 (+ SocketIndex _returnvalue_5))
  ;[1 1 1] Tries to attach a limb with the given preferred index to the given player
  (bind _socketinuse (CallFunction|SocketStatus _haslimb SocketIndex))
  (if _socketinuse
    (if (!= SocketIndex 0)
      (bind _socketinuse_2 (CallFunction|SocketStatus _haslimb _returnvalue_7))
      (if _socketinuse_2
        ;[1 1 1] Allow legs to go in arm sockets if both leg sockets are full
        (if (>= SocketIndex 3)
          (bind _socketinuse_3 (CallFunction|SocketStatus _haslimb _returnvalue_4))
          (if _socketinuse_3
            (bind _socketinuse_4 (CallFunction|SocketStatus _haslimb _returnvalue_6))
            (if (not _socketinuse_4)
              (CallFunction|AttachLimbEvent _returnvalue_6 Player))
            (else
              (CallFunction|AttachLimbEvent _returnvalue_4 Player))))
        (else
          (CallFunction|AttachLimbEvent _returnvalue_7 Player))))
    (else
      (CallFunction|AttachLimbEvent SocketIndex Player))))

(event Custom|AttachLimbEvent
  (params (SocketIndex :type Integer) (ToPlayer :type Skele%20BP%20Object%20Reference))
  ;[1 1 1] Update variables to tell the server the limb's attached
  (Utilities|Array|SetArrayElem (Variables|/Game/SkeletonWar/Blueprints/PlayerCharacters/Skele_BP.Skele_BP_C|GetLimbs ToPlayer) SocketIndex self true)
  (Utilities|Array|SetArrayElem (Variables|/Game/SkeletonWar/Blueprints/PlayerCharacters/Skele_BP.Skele_BP_C|GetHasLimb ToPlayer) SocketIndex true)
  (bind _output_get (Variables|Default|SetActualSocketIndex SocketIndex))
  (Variables|Default|SetLimbParentPlayer ToPlayer)
  (Variables|Default|SetIsAttached true)
  (Networking|SwitchHasAuthority
    (:Authority
      (CallFunction|AttachLimbSound))))

(event Custom|PlayerOverlapDetection
  (params (OverlappingPlayer :type Skele%20BP%20Object%20Reference))
  (Networking|SwitchHasAuthority
    (:Authority
      (if (Variables|Default|GetReadyToAttach)
        (CallFunction|AttachLimbs OverlappingPlayer (Variables|Default|GetPreferredSocketIndex))))))

(fn ConstructionScript)

(fn GetSocketName
  (bind _preferredsocketindex (Variables|Default|GetPreferredSocketIndex))
  (return (Utilities|Array|Get(acopy) (Variables|Default|GetLimbSocketNames) _preferredsocketindex) _preferredsocketindex))

(fn SocketStatus
  (params (HasLimbArray :type Array%20of%20Booleans) (SocketIndex :type Integer))
  (return (Utilities|Array|Get(acopy) HasLimbArray SocketIndex)))

(fn OnRepIsAttached
  (bind _isattached (Variables|Default|GetIsAttached))
  (Physics|SetSimulatePhysics (not _isattached))
  (if _isattached
    (Class|Actor|AttachRootComponentto (Variables|/Script/Engine.Character|GetMesh (Variables|Default|GetLimbParentPlayer)) (Utilities|Array|Get(acopy) (Variables|Default|GetLimbSocketNames) (Variables|Default|GetActualSocketIndex)) "SnapToTarget" true)
    (else
      (Class|SceneComponent|DetachfromParent true true))))

(fn SetLimbVariablesonWeaponEquip
  (params (Weapon :type Weapon%20Object%20Reference))
  (bind _limbparentplayer (Variables|Default|GetLimbParentPlayer))
  ;[1 1 1] Set variables on limb
  (Variables|Default|SetLimbWeaponEquipped Weapon)
  (Variables|Default|SetLimbHasWeapon true)
  ;[1 1 1] Set Variables on Player
  (Utilities|FlowControl|Sequence
    (:then_0
      (Variables|/Game/SkeletonWar/Blueprints/PlayerCharacters/Skele_BP.Skele_BP_C|SetPlayerHasWeapon _limbparentplayer true))
    (:then_1
      (Variables|/Game/SkeletonWar/Blueprints/PlayerCharacters/Skele_BP.Skele_BP_C|SetWeaponLimb _limbparentplayer self))
    (:then_2
      (Variables|/Game/SkeletonWar/Blueprints/PlayerCharacters/Skele_BP.Skele_BP_C|SetEquippedWeapon _limbparentplayer (Variables|Default|GetLimbWeaponEquipped)))))

(fn SetLimbVariablesonWeaponDetach
  (if (Variables|Default|GetLimbHasWeapon)
    (Variables|/Game/SkeletonWar/Blueprints/Weapons/Weapon.Weapon_C|SetIsWeaponEquipped (Variables|Default|GetLimbWeaponEquipped) false)
    (Variables|Default|SetLimbHasWeapon false)
    (Variables|/Game/SkeletonWar/Blueprints/PlayerCharacters/Skele_BP.Skele_BP_C|SetPlayerHasWeapon (Variables|Default|GetLimbParentPlayer) false)))

(fn SetAnimationState
  (bind _limbparentplayer (Variables|Default|GetLimbParentPlayer))
  (bind _haslimb (Variables|/Game/SkeletonWar/Blueprints/PlayerCharacters/Skele_BP.Skele_BP_C|GetHasLimb _limbparentplayer))
  (bind _limbs (Variables|/Game/SkeletonWar/Blueprints/PlayerCharacters/Skele_BP.Skele_BP_C|GetLimbs _limbparentplayer))
  (bind _item (Utilities|Array|Get(acopy) _haslimb 3))
  (bind _item_2 (Utilities|Array|Get(acopy) _haslimb 4))
  ;[1 1 1] Hopping
  (if (Class|KismetMathLibrary|XORBoolean _item _item_2)
    (Variables|Default|SetAnimState "NewEnumerator1")
    (else
      ;[1 1 1] Crawling
      (if (and (not _item_2) (not _item))
        (Variables|Default|SetAnimState "NewEnumerator2")
        (else
          ;[1 1 1] If not hopping or crawling, check what types of limbs are attached
          ;;[1 1 1] AllFours
          (if (Math|Boolean|ANDBoolean (CallFunction|IsLeg? _limbs "NewEnumerator2") (CallFunction|IsLeg? _limbs "NewEnumerator1") (CallFunction|IsLeg? _limbs "NewEnumerator3") (CallFunction|IsLeg? _limbs "NewEnumerator4"))
            (Variables|Default|SetAnimState "NewEnumerator4")
            (else
              ;;[1 1 1] Cartwheeling
              (if (Math|Boolean|ANDBoolean (CallFunction|IsArm? _limbs "NewEnumerator2") (CallFunction|IsArm? _limbs "NewEnumerator1") (CallFunction|IsArm? _limbs "NewEnumerator3") (CallFunction|IsArm? _limbs "NewEnumerator4"))
                (Variables|Default|SetAnimState "NewEnumerator2")
                (else
                  (Variables|Default|SetAnimState "NewEnumerator0"))))))))))

(fn LimbApplyImpulse
  (Physics|AddImpulse (Math|Vector|MakeVector (Math|Random|RandomFloatinRange -2e+03 2e+03) (Math|Random|RandomFloatinRange -2e+03 2e+03) 1.5e+03) "None" true))