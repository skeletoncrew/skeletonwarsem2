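; Skeleton War game mode that handles player login, respawning and Rubix-mode colour assignment, with server authority.
; Login applies GameInstance server settings on first join, numbers players and sends those over the limit to spectate.
; Respawn spawns a Skele_BP at the PlayerStart farthest from its nearest skeleton.
; Rubix colours follow player number; limbs get other players' colours or, during first setup, can swap through per-body-part non-matching limb arrays.
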(event Custom|Respawn
  (params (Controller :type Player%20Controller%20Object%20Reference))
  ;[1 1 1] Pick a respawn point and possess a new pawn
  (Utilities|IsValid Controller
    (:Is%20Valid
      (Networking|SwitchHasAuthority
        (:Authority
          (bind _transform (CallFunction|GetSafestRespawnPoint))
          (bind _returnvalue (Game|SpawnActorfromClass "/Game/SkeletonWar/Blueprints/PlayerCharacters/Skele_BP.Skele_BP_C" _transform true Controller 0))
          (Utilities|IsValid _returnvalue
            (:Is%20Valid
              (Pawn|Possess Controller _returnvalue)
              (Default|SetOverheadText _returnvalue))))))))

(event EventPostLogin
  (params (NewPlayer :type Player%20Controller%20Object%20Reference))
  ;[1 1 1] Set the player's name and call the PostLogin event
  (Networking|SwitchHasAuthority
    (:Authority
      (bind _asskele_player_controller (Utilities|Casting|CastToSkele_PlayerController NewPlayer))
      (bind _asskele_game_instance (Utilities|Casting|CastToSkele_GameInstance (Game|GetGameInstance)))
      (if (> (Variables|Default|GetNumPlayers) (.MaxPlayers (Utilities|Struct|BreakServerSettings_Struct (Variables|/Game/SkeletonWar/Blueprints/Skele_GameInstance.Skele_GameInstance_C|GetServerSettings _asskele_game_instance))))
        (Default|EnterSpectatorMode _asskele_player_controller)
        (else
          (if (Variables|Default|GetServerHasJoined)
            _
            (else
              (bind _asskele_game_state (Utilities|Casting|CastToSkele_GameState (Game|GetGameState)))
              (Variables|/Game/SkeletonWar/Blueprints/Skele_GameState.Skele_GameState_C|SetGameEndTime _asskele_game_state (* (.GameTime (Utilities|Struct|BreakServerSettings_Struct (Variables|/Game/SkeletonWar/Blueprints/Skele_GameInstance.Skele_GameInstance_C|GetServerSettings _asskele_game_instance))) 6e+01))
              (Variables|/Game/SkeletonWar/Blueprints/Skele_GameState.Skele_GameState_C|SetServerName _asskele_game_state (.ServerName (Utilities|Struct|BreakServerSettings_Struct (Variables|/Game/SkeletonWar/Blueprints/Skele_GameInstance.Skele_GameInstance_C|GetServerSettings _asskele_game_instance))))
              (Variables|Default|SetGameMode (.GameMode (Utilities|Struct|BreakServerSettings_Struct (Variables|/Game/SkeletonWar/Blueprints/Skele_GameInstance.Skele_GameInstance_C|GetServerSettings _asskele_game_instance))))
              (Variables|Default|SetServerHasJoined true)))
          (Variables|/Game/SkeletonWar/Blueprints/Skele_PlayerController.Skele_PlayerController_C|SetPlayerNumber _asskele_player_controller (Variables|Default|GetNumPlayers))
          (Default|ClientPostLogin _asskele_player_controller))))))

(event Custom|AssignColour
  (params (Bone :type Actor%20Object%20Reference))
  ;[1 1 1] If it's rubix mode set colour
  (Networking|SwitchHasAuthority
    (:Authority
      (if (Utilities|Enum|Equal(Enum) (Variables|Default|GetGameMode) "NewEnumerator1")
        (CallFunction|SetColour Bone)))))

(fn ConstructionScript)

(fn SetColour
  (params (Actor :type Actor%20Object%20Reference))
  (bind _numplayers (Variables|Default|GetNumPlayers))
  (bind _arrayofints (Variables|Default|GetArrayofInts))
  (bind _asskele_bp (Utilities|Casting|CastToSkele_BP Actor)
    (:then
      (bind _asskele_player_controller (Utilities|Casting|CastToSkele_PlayerController (Components|GetOwner _asskele_bp)))
      (Variables|Default|SetTempPlayerController _asskele_player_controller)
      (Variables|/Game/SkeletonWar/Blueprints/PlayerCharacters/Skele_BP.Skele_BP_C|SetColourIndex _asskele_bp (- (Variables|/Game/SkeletonWar/Blueprints/Skele_PlayerController.Skele_PlayerController_C|GetPlayerNumber _asskele_player_controller) 1))
      (Variables|Rubix|SetTempPlayerColourIndex (- (Variables|/Game/SkeletonWar/Blueprints/Skele_PlayerController.Skele_PlayerController_C|GetPlayerNumber _asskele_player_controller) 1)))
    (:CastFailed
      (bind _aslimb (Utilities|Casting|CastToLimb Actor))
      (if (Variables|/Game/SkeletonWar/Blueprints/Skele_PlayerController.Skele_PlayerController_C|GetFirstSetupComplete (Variables|Default|GetTempPlayerController))
        (Utilities|Array|RemoveItem _arrayofints (Variables|Rubix|GetTempPlayerColourIndex))
        (Variables|/Game/SkeletonWar/Blueprints/Limbs/Limb.Limb_C|SetColourIndex _aslimb (Utilities|Array|Get(acopy) _arrayofints (Math|Random|RandomIntegerinRange 0 (- (Variables|Default|GetNumPlayers) 2))))
        (Utilities|Array|Insert _arrayofints (Variables|Rubix|GetTempPlayerColourIndex) (Variables|Rubix|GetTempPlayerColourIndex))
        (elif (== _numplayers 1)
          (Variables|/Game/SkeletonWar/Blueprints/Limbs/Limb.Limb_C|SetColourIndex _aslimb 1)
          (elif (== _numplayers 2)
            (Variables|/Game/SkeletonWar/Blueprints/Limbs/Limb.Limb_C|SetColourIndex _aslimb 0)
            (elif (>= _numplayers 3)
              (if (< (Utilities|Array|Length (Variables|Rubix|GetNonMatchingLimbs)) 1)
                (Variables|/Game/SkeletonWar/Blueprints/Limbs/Limb.Limb_C|SetColourIndex _aslimb (Variables|Rubix|GetTempPlayerColourIndex))
                (else
                  (bind (_head _leftarm _rightarm _leftleg _rightleg) (CallFunction|LimbClass _aslimb))
                  (if _head
                    (CallFunction|SetIndexfromNonMatchingLimbArray _aslimb (Variables|Rubix|GetHead))
                    (elif _leftarm
                      (CallFunction|SetIndexfromNonMatchingLimbArray _aslimb (Variables|Rubix|GetLeftArm))
                      (elif _rightarm
                        (CallFunction|SetIndexfromNonMatchingLimbArray _aslimb (Variables|Rubix|GetRightArm))
                        (elif _leftleg
                          (CallFunction|SetIndexfromNonMatchingLimbArray _aslimb (Variables|Rubix|GetLeftLeg))
                          (elif _rightleg
                            (CallFunction|SetIndexfromNonMatchingLimbArray _aslimb (Variables|Rubix|GetRightLeg))))))))))))))))

(fn SetIndexfromNonMatchingLimbArray
  (params (Limb :type Limb%20Object%20Reference) (NonMatchingLimbArray :type Array%20of%20Limb%20Object%20References))
  (if (Utilities|ArrayNotEmpty NonMatchingLimbArray)
    (bind _output_get (Variables|Rubix|SetTempArrayIndex (Math|Random|RandomInteger (Utilities|Array|Length NonMatchingLimbArray))))
    (bind _output_get_2 (Variables|Rubix|SetTempColourIndex (Variables|/Game/SkeletonWar/Blueprints/Limbs/Limb.Limb_C|GetColourIndex (Utilities|Array|Get(acopy) NonMatchingLimbArray _output_get))))
    (Variables|/Game/SkeletonWar/Blueprints/Limbs/Limb.Limb_C|SetColourIndex (Utilities|Array|Get(acopy) NonMatchingLimbArray _output_get) (Variables|Rubix|GetTempPlayerColourIndex))
    (Variables|/Game/SkeletonWar/Blueprints/Limbs/Limb.Limb_C|SetColourIndex Limb _output_get_2)
    (else
      (Variables|/Game/SkeletonWar/Blueprints/Limbs/Limb.Limb_C|SetColourIndex Limb (Variables|Rubix|GetTempPlayerColourIndex)))))

(fn AddtoNonMatchingLimbArrays
  (params (Limb :type Limb%20Object%20Reference))
  (bind _nonmatchinglimbs (Variables|Rubix|GetNonMatchingLimbs))
  (if (not (Utilities|Array|ContainsItem _nonmatchinglimbs Limb))
    (Utilities|Array|Add _nonmatchinglimbs Limb)
    (bind (_head _leftarm _rightarm _leftleg _rightleg) (CallFunction|LimbClass Limb))
    (if _head
      (Utilities|Array|Add (Variables|Rubix|GetHead) Limb)
      (elif _leftarm
        (Utilities|Array|Add (Variables|Rubix|GetLeftArm) Limb)
        (elif _rightarm
          (Utilities|Array|Add (Variables|Rubix|GetRightArm) Limb)
          (elif _leftleg
            (Utilities|Array|Add (Variables|Rubix|GetLeftLeg) Limb)
            (elif _rightleg
              (Utilities|Array|Add (Variables|Rubix|GetRightLeg) Limb))))))))

(fn RemovefromNonMatchingLimbArrays
  (params (Limb :type Limb%20Object%20Reference))
  (bind _nonmatchinglimbs (Variables|Rubix|GetNonMatchingLimbs))
  (if (Utilities|Array|ContainsItem _nonmatchinglimbs Limb)
    (Utilities|Array|RemoveItem _nonmatchinglimbs Limb)
    (bind (_head _leftarm _rightarm _leftleg _rightleg) (CallFunction|LimbClass Limb))
    (if _head
      (Utilities|Array|RemoveItem (Variables|Rubix|GetHead) Limb)
      (elif _leftarm
        (Utilities|Array|RemoveItem (Variables|Rubix|GetLeftArm) Limb)
        (elif _rightarm
          (Utilities|Array|RemoveItem (Variables|Rubix|GetRightArm) Limb)
          (elif _leftleg
            (Utilities|Array|RemoveItem (Variables|Rubix|GetLeftLeg) Limb)
            (elif _rightleg
              (Utilities|Array|RemoveItem (Variables|Rubix|GetRightLeg) Limb))))))))

(fn GetSafestRespawnPoint
  (Utilities|Array|Clear (LocalVariables|GetDistances))
  (Utilities|Array|Clear (LocalVariables|GetSafestRespawns))
  (bind _outactors (Actor|GetAllActorsOfClass "/Script/Engine.PlayerStart"))
  (for (_array_element _array_index) _outactors
    (Utilities|Array|Add (LocalVariables|GetDistances) 1e+05)
    (Utilities|Array|Add (LocalVariables|GetSafestRespawns) (Transformation|GetActorTransform _array_element))
    (bind _outactors_2 (Actor|GetAllActorsOfClass "/Game/SkeletonWar/Blueprints/PlayerCharacters/Skele_BP.Skele_BP_C"))
    (if (<= (Utilities|Array|Length _outactors_2) 0)
      ;[1 1 1] Just choose a random spawn if there's only one player on the map
      (LocalVariables|SetSafestRespawn (Transformation|GetActorTransform (Utilities|Array|Get(acopy) _outactors (Math|Random|RandomInteger (Utilities|Array|Length _outactors)))))
      (return (LocalVariables|GetSafestRespawn))
      (else
        (for _array_element_2 _outactors_2
          (if (< (Transformation|GetDistanceTo _array_element _array_element_2) (Utilities|Array|Get(acopy) (LocalVariables|GetDistances) _array_index))
            (Utilities|Array|SetArrayElem (LocalVariables|GetDistances) _array_index (Transformation|GetDistanceTo _array_element _array_element_2)))))))
  (LocalVariables|SetSafestRespawn (Utilities|Array|Get(acopy) (LocalVariables|GetSafestRespawns) (.IndexOfMaxValue (Math|Float|MaxOfFloatArray (LocalVariables|GetDistances)))))
  (return (LocalVariables|GetSafestRespawn)))

(fn LimbClass
  (params (Limb :type Limb%20Object%20Reference))
  (bind _returnvalue (Utilities|GetClass Limb))
  (return (== _returnvalue "/Game/SkeletonWar/Blueprints/Limbs/Head_BP.Head_BP_C") (== _returnvalue "/Game/SkeletonWar/Blueprints/Limbs/LeftArm_BP.LeftArm_BP_C") (== _returnvalue "/Game/SkeletonWar/Blueprints/Limbs/RightArm_BP.RightArm_BP_C") (== _returnvalue "/Game/SkeletonWar/Blueprints/Limbs/LeftLeg_BP.LeftLeg_BP_C") (== _returnvalue "/Game/SkeletonWar/Blueprints/Limbs/RightLeg_BP.RightLeg_BP_C")))